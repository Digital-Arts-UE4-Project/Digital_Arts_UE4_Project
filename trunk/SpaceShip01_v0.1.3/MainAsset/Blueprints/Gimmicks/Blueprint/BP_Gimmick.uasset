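; Base gimmick Blueprint that switches on or off according to how much energy it holds.
; AddEnergy and SubEnergy step the Energy count by one, then set IsEnergy by comparing it to FullEnergy.
; IsActive inverts the response: when false, full energy turns the gimmick on; when true, full energy turns it off.
; Its Gimmick_ON and Gimmick_OFF events are empty, leaving the actual effect undefined here.
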(event Custom|AddEnergy
  ;[1 1 1] ギミックのON/OFF
  (Variables|Default|SetEnergy (+ (Variables|Default|GetEnergy) 1))
  (Variables|Default|SetIsEnergy (<= (Variables|Default|GetFullEnergy) (Variables|Default|GetEnergy)))
  (if (Variables|Default|GetIsActive)
    (if (Variables|Default|GetIsEnergy)
      (CallFunction|GimmickOFF :!label _label)
      (else
        (CallFunction|GimmickON :!label _label_2)))
    (elif (Variables|Default|GetIsEnergy)
      (goto _label_2)
      (else
        (goto _label)))))

(event Custom|SubEnergy
  ;[1 1 1] ギミックのON/OFF
  (Variables|Default|SetEnergy (- (Variables|Default|GetEnergy) 1))
  (Variables|Default|SetIsEnergy (<= (Variables|Default|GetFullEnergy) (Variables|Default|GetEnergy)))
  (if (Variables|Default|GetIsActive)
    (if (Variables|Default|GetIsEnergy)
      (CallFunction|GimmickOFF :!label _label)
      (else
        (CallFunction|GimmickON :!label _label_2)))
    (elif (Variables|Default|GetIsEnergy)
      (goto _label_2)
      (else
        (goto _label)))))

(event Custom|Gimmick_ON
  ;[1 1 1] ギミックのON/OFF
)

(event Custom|Gimmick_OFF
  ;[1 1 1] ギミックのON/OFF
)

(fn ConstructionScript)