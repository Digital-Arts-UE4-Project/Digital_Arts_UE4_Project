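; BP_EnergySpawner is a gimmick actor that spawns a BP_Energy at an offset from its location and shows a particle and light effect.
; It spawns one on BeginPlay and sets itself as that energy's Spawner reference.
; DisappearEnergy switches off the particles and light, while RespawnEnergy spawns a new energy and restores both.
; The construction script applies LightPower to the point light.
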(event Custom|Respawn%20Energy
  (CallFunction|Spawn)
  (Components|Activation|SetActive (Variables|Default|GetParticleSystem) true false)
  (Rendering|Components|Light|SetIntensity (Variables|Default|GetPointLight) (Variables|Default|GetLightPower)))

(event Custom|Disappear%20Energy
  (Components|Activation|SetActive (Variables|Default|GetParticleSystem) false false)
  (Rendering|Components|Light|SetIntensity (Variables|Default|GetPointLight) 0.0))

(event EventBeginPlay
  (CallFunction|Spawn))

(fn ConstructionScript
  (Rendering|Components|Light|SetIntensity (Variables|Default|GetPointLight) (Variables|Default|GetLightPower)))

(fn Spawn
  (bind _returnvalue (Game|SpawnActorfromClass "/Game/MainAsset/Blueprints/Gimmicks/Blueprint/BP_Energy.BP_Energy_C" (Math|Conversions|ToTransform(Vector) (+ (Transformation|GetActorLocation) (Variables|Default|GetSpawnPoint))) "Undefined" 0 0))
  (Variables|/Game/MainAsset/Blueprints/Gimmicks/Blueprint/BP_Energy.BP_Energy_C|SetSpawner _returnvalue self)
  (return))