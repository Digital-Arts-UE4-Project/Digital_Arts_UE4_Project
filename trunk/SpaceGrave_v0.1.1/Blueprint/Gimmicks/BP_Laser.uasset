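; Laser barrier gimmick with two poles and a vertical stack of beams that can be switched on or off.
; The construction script spaces and stretches the poles from Width and Height.
; BeginPlay spawns LaserCount BP_LaserLine actors spread over the height, scaled to the width and nudged inward at the ends, then applies IsActive.
; The gimmick ON/OFF events only activate or deactivate each stored line's particle system.
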(event Custom|Gimmick_ON
  ;[1 1 1] ギミックのON/OFF
  (for _array_element (Variables|Default|GetLaserArrey)
    (Components|Activation|Activate (Variables|/Game/Blueprint/Gimmicks/Blueprint/BP_LaserLine.BP_LaserLine_C|GetParticleSystem _array_element) false)))

(event Custom|Gimmick_OFF
  ;[1 1 1] ギミックのON/OFF
  (for _array_element (Variables|Default|GetLaserArrey)
    (Components|Activation|Deactivate (Variables|/Game/Blueprint/Gimmicks/Blueprint/BP_LaserLine.BP_LaserLine_C|GetParticleSystem _array_element))))

(event EventBeginPlay
  (bind _returnvalue (Transformation|GetActorTransform))
  ;[1 1 1] 初期設定
  (Variables|Default|SetLaserCount (- (Variables|Default|GetLaserCount) 1.0))
  (for _index (range 0 (Math|Float|Truncate (Variables|Default|GetLaserCount)))
    (if (<= _index 0)
      (Variables|Default|SetOffset 2.0)
      (elif (>= _index (Math|Float|Truncate (Variables|Default|GetLaserCount)))
        (Variables|Default|SetOffset -2.0)))
    (bind _returnvalue_2 (Game|SpawnActorfromClass "/Game/Blueprint/Gimmicks/Blueprint/BP_LaserLine.BP_LaserLine_C" (Math|Transform|MakeTransform (Math|Vector|MakeVector (.x (.location _returnvalue)) (.y (.location _returnvalue)) (+ (* (Math|Conversions|ToFloat(Integer) _index) (/ (* (Variables|Default|GetHeight) 2e+02) (Variables|Default|GetLaserCount))) (.z (.location _returnvalue)) (Variables|Default|GetOffset))) (.rotation _returnvalue) (Math|Vector|MakeVector (/ (Variables|Default|GetWidth) 2.0) (.y (.scale _returnvalue)) (.z (.scale _returnvalue)))) "Undefined" 0 0))
    (Utilities|Array|Add (Variables|Default|GetLaserArrey) _returnvalue_2))
  (if (Variables|Default|GetIsActive)
    (CallFunction|GimmickON)
    (else
      (CallFunction|GimmickOFF))))

(fn ConstructionScript
  (bind _sm_leftpole (Variables|Default|GetSM_LeftPole))
  (bind _sm_rightpole (Variables|Default|GetSM_RightPole))
  (bind _width (Variables|Default|GetWidth))
  (bind _returnvalue (Transformation|GetRelativeTransform _sm_rightpole))
  (bind _returnvalue_2 (Transformation|GetRelativeTransform _sm_leftpole))
  (bind _returnvalue_3 (* _width 1e+02))
  (bind _returnvalue_4 (+ _returnvalue_3 -5.0))
  (Utilities|FlowControl|Sequence
    (:then_0
      (Transformation|SetRelativeTransform _sm_leftpole (Math|Transform|MakeTransform (Math|Vector|MakeVector _returnvalue_4 (.y (.location _returnvalue_2)) (.z (.location _returnvalue_2))) (.rotation _returnvalue_2) (Math|Vector|MakeVector (.x (.scale _returnvalue_2)) (.y (.scale _returnvalue_2)) (Variables|Default|GetHeight))) false false))
    (:then_1
      (Transformation|SetRelativeTransform _sm_rightpole (Math|Transform|MakeTransform (Math|Vector|MakeVector (* _returnvalue_4 -1.0) (.y (.location _returnvalue)) (.z (.location _returnvalue))) (.rotation _returnvalue) (Math|Vector|MakeVector (.x (.scale _returnvalue)) (.y (.scale _returnvalue)) (Variables|Default|GetHeight))) false false))))