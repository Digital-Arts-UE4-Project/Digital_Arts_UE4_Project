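; BP_CrystalCapsule is a breakable glass capsule that comes with a crystal.
; On BeginPlay it spawns a scaled BP_Crystal above its own location and gives its destructible mesh the crystal glass material.
; The Break event swaps that material to plain glass, then applies damage with an impulse at the mesh location to shatter the capsule.
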(event Custom|Break
  (bind _sm_capsule_dm (Variables|Default|GetSM_Capsule_DM))
  ;[1 1 1] ガラスが割れる
  (Rendering|Material|SetMaterial _sm_capsule_dm 0 "/Game/StarterContent/Materials/M_Glass.M_Glass")
  (Game|Damage|ApplyDamage _sm_capsule_dm 1e+02 (Transformation|GetWorldLocation _sm_capsule_dm) (Math|Vector|MakeVector 1e+02 1e+02 1e+02) 5.0))

(event EventBeginPlay
  (bind _returnvalue (Transformation|GetActorTransform))
  ;[1 1 1] 初期設定
  (Game|SpawnActorfromClass "/Game/Blueprint/Object/Blueprint/BP_Crystal.BP_Crystal_C" (Math|Transform|MakeTransform (Math|Vector|MakeVector (.x (.location _returnvalue)) (.y (.location _returnvalue)) (+ (.z (.location _returnvalue)) 2e+02)) (.rotation _returnvalue) "0.800000,0.800000,1") "Undefined" 0 0)
  (Rendering|Material|SetMaterial (Variables|Default|GetSM_Capsule_DM) 0 "/Game/Blueprint/Object/Material/M_CrystalGlass.M_CrystalGlass"))

(fn ConstructionScript)