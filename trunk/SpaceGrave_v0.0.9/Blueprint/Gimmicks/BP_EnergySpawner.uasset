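; BP_EnergySpawner is a gimmick that spawns a BP_Energy actor at an offset from its own location and shows whether it is active.
; It spawns one on BeginPlay and sets itself as that actor's Spawner reference.
; DisappearEnergy switches off the particle system, light and IsActive flag, while RespawnEnergy spawns a new energy and restores them.
; The construction script applies LightPower to the point light.
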(event Custom|Respawn%20Energy
  (CallFunction|Spawn)
  (Components|Activation|SetActive (Variables|Default|GetParticleSystem) true false)
  (Rendering|Components|Light|SetIntensity (Variables|Default|GetPointLight) (Variables|Default|GetLightPower))
  (Variables|Default|SetIsActive true))

(event Custom|Disappear%20Energy
  (Components|Activation|SetActive (Variables|Default|GetParticleSystem) false false)
  (Rendering|Components|Light|SetIntensity (Variables|Default|GetPointLight) 0.0)
  (Variables|Default|SetIsActive false))

(event EventBeginPlay
  (CallFunction|Spawn))

(fn ConstructionScript
  (Rendering|Components|Light|SetIntensity (Variables|Default|GetPointLight) (Variables|Default|GetLightPower)))

(fn Spawn
  (bind _returnvalue (Game|SpawnActorfromClass "/Game/Blueprint/Gimmicks/Blueprint/BP_Energy.BP_Energy_C" (Math|Conversions|ToTransform(Vector) (+ (Transformation|GetActorLocation) (Variables|Default|GetSpawnPoint))) "Undefined" 0 0))
  (Variables|/Game/Blueprint/Gimmicks/Blueprint/BP_Energy.BP_Energy_C|SetSpawner _returnvalue self)
  (return))