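; Gimmick wall made of a row of mesh segments that slide along a chosen axis when switched on and back when switched off.
; The construction script builds the segments from length, size and direction, and places a Box previewing their destination.
; A Slow or Normal timeline moves one segment at a time, stepping through the array and reversing order on Gimmick_OFF.
; If IsActive, BeginPlay starts all segments at the moved position.
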(event Custom|WallMove
  (bind _wallarray (Variables|Default|GetWallArray))
  (bind _count (Variables|Default|GetCount))
  (bind _wallarray_2 (Variables|Default|GetWallArray))
  (bind _count_2 (Variables|Default|GetCount))
  (bind _wallarray_3 (Variables|Default|GetWallArray))
  (bind _count_3 (Variables|Default|GetCount))
  (bind _item (Utilities|Array|Get(acopy) _wallarray _count))
  (bind _item_2 (Utilities|Array|Get(acopy) _wallarray_2 _count_2))
  (bind _item_3 (Utilities|Array|Get(acopy) _wallarray_3 _count_3))
  (bind _relativelocation (Variables|/Script/Engine.SceneComponent|GetRelativeLocation _item))
  (bind _relativelocation_2 (Variables|/Script/Engine.SceneComponent|GetRelativeLocation _item_2))
  (bind _relativelocation_3 (Variables|/Script/Engine.SceneComponent|GetRelativeLocation _item_3))
  ;[1 1 1] 動作
  (switch Utilities|FlowControl|Switch|SwitchonE_WallVector (Variables|Default|GetMoveDirection)
    (:NewEnumerator0
      (switch Utilities|FlowControl|Switch|SwitchonE_WallVector (Variables|Default|GetWallDirection)
        (:NewEnumerator0
          (Variables|Default|SetPosition (+ (* (* (Variables|Default|GetCount) (Variables|Default|GetWallSize)) 2e+02) (Variables|Default|GetPosition))))
        (:NewEnumerator1
          _)
        (:NewEnumerator2
          _))
      (Transformation|SetRelativeLocation _item (Math|Vector|MakeVector (Variables|Default|GetPosition) (.y _relativelocation) (.z _relativelocation)) false false))
    (:NewEnumerator1
      (switch Utilities|FlowControl|Switch|SwitchonE_WallVector (Variables|Default|GetWallDirection)
        (:NewEnumerator0
          _)
        (:NewEnumerator1
          (Variables|Default|SetPosition (+ (* (* (Variables|Default|GetCount) (Variables|Default|GetWallSize)) 2e+02) (Variables|Default|GetPosition))))
        (:NewEnumerator2
          _))
      (Transformation|SetRelativeLocation _item_2 (Math|Vector|MakeVector (.x _relativelocation_2) (Variables|Default|GetPosition) (.z _relativelocation_2)) false false))
    (:NewEnumerator2
      (switch Utilities|FlowControl|Switch|SwitchonE_WallVector (Variables|Default|GetWallDirection)
        (:NewEnumerator0
          _)
        (:NewEnumerator1
          _)
        (:NewEnumerator2
          (Variables|Default|SetPosition (+ (* (* (Variables|Default|GetCount) (Variables|Default|GetWallSize)) 2e+02) (Variables|Default|GetPosition)))))
      (Transformation|SetRelativeLocation _item_3 (Math|Vector|MakeVector (.x _relativelocation_3) (.y _relativelocation_3) (Variables|Default|GetPosition)) false false))))

(event Custom|Gimmick_ON
  (bind _walllength (Variables|Default|GetWallLength))
  (bind _returnvalue (- _walllength 1))
  ;[1 1 1] 速さSlow/Noamlの選択
  (Variables|Default|SetMoveGo true)
  (if (Variables|Default|GetMoveSlow)
    (bind _move (Timeline|Slow_TimeLine Play)
      (:Update
        (Variables|Default|SetPosition (* _move (Variables|Default|GetMoveLength)))
        (CallFunction|WallMove :!label _label))
      (:Finished
        ;;[1 0.751 0.2201] 動かすWallの切り替え
        (if (Variables|Default|GetMoveGo) :!label _label_2
          (Variables|Default|SetCount (+ (Variables|Default|GetCount) 1))
          (else
            (Variables|Default|SetCount (- (Variables|Default|GetCount) 1))))
        (if (<= (Variables|Default|GetCount) _returnvalue)
          (if (>= (Variables|Default|GetCount) 0)
            (if (Variables|Default|GetMoveSlow)
              (if (Variables|Default|GetMoveGo)
                (Timeline|Slow_TimeLine PlayFromStart)
                (else
                  (Timeline|Slow_TimeLine ReverseFromEnd)))
              (elif (Variables|Default|GetMoveGo)
                (bind _move_2 (Timeline|Normal_TimeLine PlayFromStart)
                  (:Update
                    (Variables|Default|SetPosition (* _move_2 (Variables|Default|GetMoveLength)))
                    (goto _label))
                  (:Finished
                    (goto _label_2)))
                (else
                  (Timeline|Normal_TimeLine ReverseFromEnd))))
            (else
              (Variables|Default|SetCount 0)))
          (else
            (Variables|Default|SetCount _returnvalue)))))
    (else
      (Timeline|Normal_TimeLine Play))))

(event Custom|Gimmick_OFF
  (bind _walllength (Variables|Default|GetWallLength))
  (bind _returnvalue (- _walllength 1))
  ;[1 1 1] 速さSlow/Noamlの選択
  (Variables|Default|SetMoveGo false)
  (if (Variables|Default|GetMoveSlow)
    (bind _move (Timeline|Slow_TimeLine Reverse)
      (:Update
        (Variables|Default|SetPosition (* _move (Variables|Default|GetMoveLength)))
        (CallFunction|WallMove :!label _label))
      (:Finished
        ;;[1 0.751 0.2201] 動かすWallの切り替え
        (if (Variables|Default|GetMoveGo) :!label _label_2
          (Variables|Default|SetCount (+ (Variables|Default|GetCount) 1))
          (else
            (Variables|Default|SetCount (- (Variables|Default|GetCount) 1))))
        (if (<= (Variables|Default|GetCount) _returnvalue)
          (if (>= (Variables|Default|GetCount) 0)
            (if (Variables|Default|GetMoveSlow)
              (if (Variables|Default|GetMoveGo)
                (Timeline|Slow_TimeLine PlayFromStart)
                (else
                  (Timeline|Slow_TimeLine ReverseFromEnd)))
              (elif (Variables|Default|GetMoveGo)
                (bind _move_2 (Timeline|Normal_TimeLine PlayFromStart)
                  (:Update
                    (Variables|Default|SetPosition (* _move_2 (Variables|Default|GetMoveLength)))
                    (goto _label))
                  (:Finished
                    (goto _label_2)))
                (else
                  (Timeline|Normal_TimeLine ReverseFromEnd))))
            (else
              (Variables|Default|SetCount 0)))
          (else
            (Variables|Default|SetCount _returnvalue)))))
    (else
      (Timeline|Normal_TimeLine Reverse))))

(event EventBeginPlay
  ;[1 1 1] Activeなら初期位置を予測位置に移動
  (if (Variables|Default|GetIsActive)
    (for _index (range 0 (- (Variables|Default|GetWallLength) 1))
      (Variables|Default|SetCount _index)
      (Variables|Default|SetPosition (* 2e+02 (Variables|Default|GetMoveLength)))
      (CallFunction|WallMove))))

(fn ConstructionScript
  (bind _wallsize (Variables|Default|GetWallSize))
  (bind _walllength (Variables|Default|GetWallLength))
  (bind _wallsize_2 (Variables|Default|GetWallSize))
  (bind _wallsize_3 (Variables|Default|GetWallSize))
  (bind _wallsize_4 (Variables|Default|GetWallSize))
  (bind _movelength (Variables|Default|GetMoveLength))
  (bind _returnvalue (Math|Vector|MakeVector _wallsize_4 _wallsize_4 _wallsize_4))
  (bind _returnvalue_2 (- _walllength 1))
  (bind _returnvalue_3 (* _movelength 2e+02))
  (bind _returnvalue_4 (* _wallsize 1e+02))
  (bind _returnvalue_5 (* _returnvalue 2.0))
  (bind _returnvalue_6 (* _returnvalue_2 1e+02))
  (bind _returnvalue_7 (* _returnvalue_5 1.56))
  (bind _returnvalue_8 (* _returnvalue_6 _wallsize_2))
  (bind (_x _y _z) (Math|Vector|BreakVector _returnvalue_7))
  (bind (_x_2 _y_2 _z_2) (Math|Vector|BreakVector _returnvalue_7))
  (bind (_x_3 _y_3 _z_3) (Math|Vector|BreakVector _returnvalue_7))
  (Utilities|FlowControl|Sequence
    (:then_0
      ;[1 1 1] WallそれぞれのTransform作成
      (for _index (range 0 (- (Variables|Default|GetWallLength) 1))
        (switch Utilities|FlowControl|Switch|SwitchonE_WallVector (Variables|Default|GetWallDirection)
          (:NewEnumerator0
            (Variables|Default|SetLocation (Math|Vector|MakeVector (* (Variables|Default|GetWallSize) 2e+02 (Math|Conversions|ToFloat(Integer) _index)) 0.0 0.0)))
          (:NewEnumerator1
            (Variables|Default|SetLocation (Math|Vector|MakeVector 0.0 (* (Variables|Default|GetWallSize) 2e+02 (Math|Conversions|ToFloat(Integer) _index)) 0.0)))
          (:NewEnumerator2
            (Variables|Default|SetLocation (Math|Vector|MakeVector 0.0 0.0 (* (Variables|Default|GetWallSize) 2e+02 (Math|Conversions|ToFloat(Integer) _index))))))
        ;[1 1 1] Wallを増やして配列の作成
        (bind _returnvalue_9 (AddComponent|AddStaticMeshComponent false (Math|Transform|MakeTransform (Variables|Default|GetLocation) "0, 0, 0" (* (Math|Vector|MakeVector _wallsize_3 _wallsize_3 _wallsize_3) 2.0))))
        (Rendering|Material|CreateDynamicMaterialInstance _returnvalue_9 0 (Variables|Default|GetMaterial) :!class /Script/Engine.PrimitiveComponent)
        (Utilities|Array|Add (Variables|Default|GetWallArray) _returnvalue_9)))
    (:then_1
      ;[1 1 1] WallDirectionに従って予測位置の大きさ決定
      (switch Utilities|FlowControl|Switch|SwitchonE_WallVector (Variables|Default|GetWallDirection)
        (:NewEnumerator0
          (Variables|Default|SetPredictedScale (Math|Vector|MakeVector (* (Variables|Default|GetWallLength) _x_2) _y_2 _z_2))
          ;[1 1 1] WallDirectionに従った予測位置の決定
          (Variables|Default|SetPredictedLocation (Math|Vector|MakeVector _returnvalue_8 0.0 0.0)))
        (:NewEnumerator1
          (Variables|Default|SetPredictedScale (Math|Vector|MakeVector _x_3 (* (Variables|Default|GetWallLength) _y_3) _z_3))
          (Variables|Default|SetPredictedLocation (Math|Vector|MakeVector 0.0 _returnvalue_8 0.0)))
        (:NewEnumerator2
          (Variables|Default|SetPredictedScale (Math|Vector|MakeVector _x _y (* (Variables|Default|GetWallLength) _z)))
          (Variables|Default|SetPredictedLocation (Math|Vector|MakeVector 0.0 0.0 _returnvalue_8)))))
    (:then_2
      ;[1 1 1] MoveDirectionに従った予測位置の決定
      (switch Utilities|FlowControl|Switch|SwitchonE_WallVector (Variables|Default|GetMoveDirection)
        (:NewEnumerator0
          (Variables|Default|SetPredictedLocation (+ (Math|Vector|MakeVector _returnvalue_3 0.0 _returnvalue_4) (Variables|Default|GetPredictedLocation))))
        (:NewEnumerator1
          (Variables|Default|SetPredictedLocation (+ (Math|Vector|MakeVector 0.0 _returnvalue_3 _returnvalue_4) (Variables|Default|GetPredictedLocation))))
        (:NewEnumerator2
          (Variables|Default|SetPredictedLocation (+ (Math|Vector|MakeVector 0.0 0.0 (+ _returnvalue_3 _returnvalue_4)) (Variables|Default|GetPredictedLocation)))))
      ;[1 1 1] 予測位置の表示
      (Transformation|SetRelativeTransform (Variables|Default|GetBox) (Math|Transform|MakeTransform (Variables|Default|GetPredictedLocation) "0, 0, 0" (Variables|Default|GetPredictedScale)) false false))))