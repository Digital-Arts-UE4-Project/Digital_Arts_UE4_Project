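; BP_Gate is a lockable sliding gate gimmick that opens when an actor enters its Box trigger, optionally only for FirstPersonCharacter.
; IsActive sets the initial lock, and GimmickON/GimmickOFF unlock or lock it, turning four door lights green or red via dynamic material instances.
; While unlocked, overlap plays a timeline that slides both halves apart and rotates the center locks; end overlap reverses it.
; While locked, overlaps neither open nor close it.
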(event OnComponentBeginOverlap(Box)
  (params (OtherActor :type Actor%20Object%20Reference) (OtherComp :type Primitive%20Component%20Object%20Reference) (OtherBodyIndex :type Integer) (bFromSweep :type Boolean) (SweepResult :type Hit%20Result%20Structure%20%28by%20ref%29))
  (bind _sm_doorlockleft (Variables|Default|GetSM_DoorLockLeft))
  (bind _sm_doorlockright (Variables|Default|GetSM_DoorLockRight))
  (bind _sm_doorlight_left (Variables|Default|GetSM_DoorLight_Left))
  (bind _sm_doorlight_right (Variables|Default|GetSM_DoorLight_Right))
  ;[0.9368 1 0.9806] 動作
  ;;[1 1 1] 作動判定(人間のみか？)
  (if (Variables|Default|GetIsHumun%20only)
    (Utilities|Casting|CastToFirstPersonCharacter OtherActor))
  ;;[1 1 1] 鍵が掛かっているか？
  (if (not (Variables|Default|GetIsLock))
    (bind (_direction _locationx _rotationy) (Timeline|Timeline_0 Play)
      (:Update
        ;;[1 1 1] 右ドア
        (Transformation|SetRelativeLocation (Variables|Default|GetSM_DoorRight) (Math|Vector|MakeVector _locationx 0.0 (Variables|Default|GetLocationZ)) false false)
        (Transformation|SetRelativeLocation (Variables|Default|GetSM_DoorLight_Big_Right) (Math|Vector|MakeVector _locationx 0.0 (Variables|Default|GetLocationZ)) false false)
        ;;[1 1 1] 左中心部
        (Transformation|SetRelativeTransform _sm_doorlockleft (Math|Transform|MakeTransform (Math|Vector|MakeVector _locationx 0.0 (Variables|Default|GetLocationZ)) (Math|Rotator|MakeRotator 0.0 (* _rotationy -1.0) 1.8e+02) (Variables|/Script/Engine.SceneComponent|GetRelativeScale3D _sm_doorlockleft)) false false)
        (Transformation|SetRelativeTransform _sm_doorlight_left (Math|Transform|MakeTransform (Math|Vector|MakeVector _locationx 0.0 (Variables|Default|GetLocationZ)) (Math|Rotator|MakeRotator 0.0 (* _rotationy -1.0) 1.8e+02) (Variables|/Script/Engine.SceneComponent|GetRelativeScale3D _sm_doorlight_left)) false false)
        ;;[1 1 1] 左ドア
        (Transformation|SetRelativeLocation (Variables|Default|GetSM_DoorLeft) (Math|Vector|MakeVector (* _locationx -1.0) 0.0 (Variables|Default|GetLocationZ)) false false)
        (Transformation|SetRelativeLocation (Variables|Default|GetSM_DoorLight_Big_Left) (Math|Vector|MakeVector (* _locationx -1.0) 0.0 (Variables|Default|GetLocationZ)) false false)
        ;;[1 1 1] 右中心部
        (Transformation|SetRelativeTransform _sm_doorlockright (Math|Transform|MakeTransform (Math|Vector|MakeVector (* _locationx -1.0) 0.0 (Variables|Default|GetLocationZ)) (Math|Rotator|MakeRotator 0.0 _rotationy 0.0) (Variables|/Script/Engine.SceneComponent|GetRelativeScale3D _sm_doorlockright)) false false)
        (Transformation|SetRelativeTransform _sm_doorlight_right (Math|Transform|MakeTransform (Math|Vector|MakeVector (* _locationx -1.0) 0.0 (Variables|Default|GetLocationZ)) (Math|Rotator|MakeRotator 0.0 _rotationy 0.0) (Variables|/Script/Engine.SceneComponent|GetRelativeScale3D _sm_doorlight_right)) false false)))))

(event OnComponentEndOverlap(Box)
  (params (OtherActor :type Actor%20Object%20Reference) (OtherComp :type Primitive%20Component%20Object%20Reference) (OtherBodyIndex :type Integer))
  (bind _sm_doorlockleft (Variables|Default|GetSM_DoorLockLeft))
  (bind _sm_doorlockright (Variables|Default|GetSM_DoorLockRight))
  (bind _sm_doorlight_left (Variables|Default|GetSM_DoorLight_Left))
  (bind _sm_doorlight_right (Variables|Default|GetSM_DoorLight_Right))
  ;[0.9368 1 0.9806] 動作
  ;;[1 1 1] 作動判定(人間のみか？)
  (if (Variables|Default|GetIsHumun%20only)
    (Utilities|Casting|CastToFirstPersonCharacter OtherActor))
  ;;[1 1 1] 鍵が掛かっているか？
  (if (not (Variables|Default|GetIsLock))
    (bind (_direction _locationx _rotationy) (Timeline|Timeline_0 Reverse)
      (:Update
        ;;[1 1 1] 右ドア
        (Transformation|SetRelativeLocation (Variables|Default|GetSM_DoorRight) (Math|Vector|MakeVector _locationx 0.0 (Variables|Default|GetLocationZ)) false false)
        (Transformation|SetRelativeLocation (Variables|Default|GetSM_DoorLight_Big_Right) (Math|Vector|MakeVector _locationx 0.0 (Variables|Default|GetLocationZ)) false false)
        ;;[1 1 1] 左中心部
        (Transformation|SetRelativeTransform _sm_doorlockleft (Math|Transform|MakeTransform (Math|Vector|MakeVector _locationx 0.0 (Variables|Default|GetLocationZ)) (Math|Rotator|MakeRotator 0.0 (* _rotationy -1.0) 1.8e+02) (Variables|/Script/Engine.SceneComponent|GetRelativeScale3D _sm_doorlockleft)) false false)
        (Transformation|SetRelativeTransform _sm_doorlight_left (Math|Transform|MakeTransform (Math|Vector|MakeVector _locationx 0.0 (Variables|Default|GetLocationZ)) (Math|Rotator|MakeRotator 0.0 (* _rotationy -1.0) 1.8e+02) (Variables|/Script/Engine.SceneComponent|GetRelativeScale3D _sm_doorlight_left)) false false)
        ;;[1 1 1] 左ドア
        (Transformation|SetRelativeLocation (Variables|Default|GetSM_DoorLeft) (Math|Vector|MakeVector (* _locationx -1.0) 0.0 (Variables|Default|GetLocationZ)) false false)
        (Transformation|SetRelativeLocation (Variables|Default|GetSM_DoorLight_Big_Left) (Math|Vector|MakeVector (* _locationx -1.0) 0.0 (Variables|Default|GetLocationZ)) false false)
        ;;[1 1 1] 右中心部
        (Transformation|SetRelativeTransform _sm_doorlockright (Math|Transform|MakeTransform (Math|Vector|MakeVector (* _locationx -1.0) 0.0 (Variables|Default|GetLocationZ)) (Math|Rotator|MakeRotator 0.0 _rotationy 0.0) (Variables|/Script/Engine.SceneComponent|GetRelativeScale3D _sm_doorlockright)) false false)
        (Transformation|SetRelativeTransform _sm_doorlight_right (Math|Transform|MakeTransform (Math|Vector|MakeVector (* _locationx -1.0) 0.0 (Variables|Default|GetLocationZ)) (Math|Rotator|MakeRotator 0.0 _rotationy 0.0) (Variables|/Script/Engine.SceneComponent|GetRelativeScale3D _sm_doorlight_right)) false false)))))

(event EventGimmickOFF
  (bind _sm_doorlight_big_right (Variables|Default|GetSM_DoorLight_Big_Right))
  (bind _sm_doorlight_big_left (Variables|Default|GetSM_DoorLight_Big_Left))
  (bind _sm_doorlight_right (Variables|Default|GetSM_DoorLight_Right))
  (bind _sm_doorlight_left (Variables|Default|GetSM_DoorLight_Left))
  ;[1 1 1] 鍵を掛ける
  (Utilities|FlowControl|Sequence
    (:then_0
      (bind _returnvalue (Rendering|Material|CreateDynamicMaterialInstance _sm_doorlight_big_right 0 (Rendering|Material|GetMaterial _sm_doorlight_big_right 0) :!class /Script/Engine.PrimitiveComponent))
      (Rendering|Material|SetVectorParameterValue _returnvalue "Light" (Variables|Default|GetCloseColor) :!class /Script/Engine.MaterialInstanceDynamic))
    (:then_1
      (bind _returnvalue_2 (Rendering|Material|CreateDynamicMaterialInstance _sm_doorlight_big_left 0 (Rendering|Material|GetMaterial _sm_doorlight_big_left 0) :!class /Script/Engine.PrimitiveComponent))
      (Rendering|Material|SetVectorParameterValue _returnvalue_2 "Light" (Variables|Default|GetCloseColor) :!class /Script/Engine.MaterialInstanceDynamic))
    (:then_2
      (bind _returnvalue_3 (Rendering|Material|CreateDynamicMaterialInstance _sm_doorlight_right 0 (Rendering|Material|GetMaterial _sm_doorlight_right 0) :!class /Script/Engine.PrimitiveComponent))
      (Rendering|Material|SetVectorParameterValue _returnvalue_3 "Light" (Variables|Default|GetCloseColor) :!class /Script/Engine.MaterialInstanceDynamic))
    (:then_3
      (bind _returnvalue_4 (Rendering|Material|CreateDynamicMaterialInstance _sm_doorlight_left 0 (Rendering|Material|GetMaterial _sm_doorlight_left 0) :!class /Script/Engine.PrimitiveComponent))
      (Rendering|Material|SetVectorParameterValue _returnvalue_4 "Light" (Variables|Default|GetCloseColor) :!class /Script/Engine.MaterialInstanceDynamic)
      (Variables|Default|SetIsLock true))))

(event EventGimmickON
  (bind _sm_doorlight_big_right (Variables|Default|GetSM_DoorLight_Big_Right))
  (bind _sm_doorlight_big_left (Variables|Default|GetSM_DoorLight_Big_Left))
  (bind _sm_doorlight_right (Variables|Default|GetSM_DoorLight_Right))
  (bind _sm_doorlight_left (Variables|Default|GetSM_DoorLight_Left))
  ;[1 1 1] 鍵を開ける
  (Utilities|FlowControl|Sequence
    (:then_0
      (bind _returnvalue (Rendering|Material|CreateDynamicMaterialInstance _sm_doorlight_big_right 0 (Rendering|Material|GetMaterial _sm_doorlight_big_right 0) :!class /Script/Engine.PrimitiveComponent))
      (Rendering|Material|SetVectorParameterValue _returnvalue "Light" (Variables|Default|GetOpenColor) :!class /Script/Engine.MaterialInstanceDynamic))
    (:then_1
      (bind _returnvalue_2 (Rendering|Material|CreateDynamicMaterialInstance _sm_doorlight_big_left 0 (Rendering|Material|GetMaterial _sm_doorlight_big_left 0) :!class /Script/Engine.PrimitiveComponent))
      (Rendering|Material|SetVectorParameterValue _returnvalue_2 "Light" (Variables|Default|GetOpenColor) :!class /Script/Engine.MaterialInstanceDynamic))
    (:then_2
      (bind _returnvalue_3 (Rendering|Material|CreateDynamicMaterialInstance _sm_doorlight_right 0 (Rendering|Material|GetMaterial _sm_doorlight_right 0) :!class /Script/Engine.PrimitiveComponent))
      (Rendering|Material|SetVectorParameterValue _returnvalue_3 "Light" (Variables|Default|GetOpenColor) :!class /Script/Engine.MaterialInstanceDynamic))
    (:then_3
      (bind _returnvalue_4 (Rendering|Material|CreateDynamicMaterialInstance _sm_doorlight_left 0 (Rendering|Material|GetMaterial _sm_doorlight_left 0) :!class /Script/Engine.PrimitiveComponent))
      (Rendering|Material|SetVectorParameterValue _returnvalue_4 "Light" (Variables|Default|GetOpenColor) :!class /Script/Engine.MaterialInstanceDynamic)
      (Variables|Default|SetIsLock false))))

(event EventBeginPlay
  (bind _sm_doorlight_big_right (Variables|Default|GetSM_DoorLight_Big_Right))
  (bind _sm_doorlight_big_left (Variables|Default|GetSM_DoorLight_Big_Left))
  (bind _sm_doorlight_right (Variables|Default|GetSM_DoorLight_Right))
  (bind _sm_doorlight_left (Variables|Default|GetSM_DoorLight_Left))
  (bind _sm_doorlight_big_right_2 (Variables|Default|GetSM_DoorLight_Big_Right))
  (bind _sm_doorlight_big_left_2 (Variables|Default|GetSM_DoorLight_Big_Left))
  (bind _sm_doorlight_right_2 (Variables|Default|GetSM_DoorLight_Right))
  (bind _sm_doorlight_left_2 (Variables|Default|GetSM_DoorLight_Left))
  ;[1 1 1] 初期設定
  (Variables|Default|SetCloseColor "(R=1.000000,G=0.000000,B=0.000000,A=1.000000)")
  (Variables|Default|SetOpenColor "(R=0.000000,G=1.000000,B=0.000000,A=1.000000)")
  (if (Variables|Default|GetIsActive)
    (Variables|Default|SetIsLock false)
    ;[1 1 1] 鍵を開ける
    (Utilities|FlowControl|Sequence
      (:then_0
        (bind _returnvalue (Rendering|Material|CreateDynamicMaterialInstance _sm_doorlight_big_right 0 (Rendering|Material|GetMaterial _sm_doorlight_big_right 0) :!class /Script/Engine.PrimitiveComponent))
        (Rendering|Material|SetVectorParameterValue _returnvalue "Light" (Variables|Default|GetOpenColor) :!class /Script/Engine.MaterialInstanceDynamic))
      (:then_1
        (bind _returnvalue_2 (Rendering|Material|CreateDynamicMaterialInstance _sm_doorlight_big_left 0 (Rendering|Material|GetMaterial _sm_doorlight_big_left 0) :!class /Script/Engine.PrimitiveComponent))
        (Rendering|Material|SetVectorParameterValue _returnvalue_2 "Light" (Variables|Default|GetOpenColor) :!class /Script/Engine.MaterialInstanceDynamic))
      (:then_2
        (bind _returnvalue_3 (Rendering|Material|CreateDynamicMaterialInstance _sm_doorlight_right 0 (Rendering|Material|GetMaterial _sm_doorlight_right 0) :!class /Script/Engine.PrimitiveComponent))
        (Rendering|Material|SetVectorParameterValue _returnvalue_3 "Light" (Variables|Default|GetOpenColor) :!class /Script/Engine.MaterialInstanceDynamic))
      (:then_3
        (bind _returnvalue_4 (Rendering|Material|CreateDynamicMaterialInstance _sm_doorlight_left 0 (Rendering|Material|GetMaterial _sm_doorlight_left 0) :!class /Script/Engine.PrimitiveComponent))
        (Rendering|Material|SetVectorParameterValue _returnvalue_4 "Light" (Variables|Default|GetOpenColor) :!class /Script/Engine.MaterialInstanceDynamic)
        (Variables|Default|SetIsLock false)))
    (else
      (Variables|Default|SetIsLock true)
      ;[1 1 1] 鍵を掛ける
      (Utilities|FlowControl|Sequence
        (:then_0
          (bind _returnvalue_5 (Rendering|Material|CreateDynamicMaterialInstance _sm_doorlight_big_right_2 0 (Rendering|Material|GetMaterial _sm_doorlight_big_right_2 0) :!class /Script/Engine.PrimitiveComponent))
          (Rendering|Material|SetVectorParameterValue _returnvalue_5 "Light" (Variables|Default|GetCloseColor) :!class /Script/Engine.MaterialInstanceDynamic))
        (:then_1
          (bind _returnvalue_6 (Rendering|Material|CreateDynamicMaterialInstance _sm_doorlight_big_left_2 0 (Rendering|Material|GetMaterial _sm_doorlight_big_left_2 0) :!class /Script/Engine.PrimitiveComponent))
          (Rendering|Material|SetVectorParameterValue _returnvalue_6 "Light" (Variables|Default|GetCloseColor) :!class /Script/Engine.MaterialInstanceDynamic))
        (:then_2
          (bind _returnvalue_7 (Rendering|Material|CreateDynamicMaterialInstance _sm_doorlight_right_2 0 (Rendering|Material|GetMaterial _sm_doorlight_right_2 0) :!class /Script/Engine.PrimitiveComponent))
          (Rendering|Material|SetVectorParameterValue _returnvalue_7 "Light" (Variables|Default|GetCloseColor) :!class /Script/Engine.MaterialInstanceDynamic))
        (:then_3
          (bind _returnvalue_8 (Rendering|Material|CreateDynamicMaterialInstance _sm_doorlight_left_2 0 (Rendering|Material|GetMaterial _sm_doorlight_left_2 0) :!class /Script/Engine.PrimitiveComponent))
          (Rendering|Material|SetVectorParameterValue _returnvalue_8 "Light" (Variables|Default|GetCloseColor) :!class /Script/Engine.MaterialInstanceDynamic)
          (Variables|Default|SetIsLock true))))))

(fn ConstructionScript)