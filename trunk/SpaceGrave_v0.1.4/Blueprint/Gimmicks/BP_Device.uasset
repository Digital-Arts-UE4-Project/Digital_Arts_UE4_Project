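; BP_Device is an energy-powered gimmick device that opens when the player enters its trigger within a set height range.
; A timeline raises the lid, pillar and floor from construction-time positions, carrying the Energy actor while active, and reverses on exit.
; DeviceActive and DeviceDeactive switch the light material and notify linked Gimmick actors through short name-based timers calling AddEnergy or SubEnergy, avoiding casts.
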(event OnComponentBeginOverlap(OpenCloseCollision)
  (params (OtherActor :type Actor%20Object%20Reference) (OtherComp :type Primitive%20Component%20Object%20Reference) (OtherBodyIndex :type Integer) (bFromSweep :type Boolean) (SweepResult :type Hit%20Result%20Structure%20%28by%20ref%29))
  (bind _returnvalue (Transformation|GetActorLocation))
  ;[1 1 1] エネルギー、スタティックメッシュの移動
  (bind _iscastplayer (CallFunction|CheckPlayer OtherActor))
  (if _iscastplayer
    (bind _locationz (Timeline|TimeLine Play)
      (:Update
        (Utilities|FlowControl|Sequence
          (:then_0
            (CallFunction|LocationMove (Variables|Default|GetLid) (Variables|SMLocation|GetLidLocation) (* _locationz 0.5)))
          (:then_1
            (CallFunction|LocationMove (Variables|Default|GetPillar) (Variables|SMLocation|GetPillarLocation) (* _locationz 0.5)))
          (:then_2
            (CallFunction|LocationMove (Variables|Default|GetMoveFloor) (Variables|SMLocation|GetFloorLocation) _locationz))
          (:then_3
            (if (Variables|Default|GetIsActive)
              (Transformation|SetActorLocation (Variables|Default|GetEnergy) (Math|Vector|MakeVector (.x _returnvalue) (.y _returnvalue) (+ (.z _returnvalue) (+ _locationz 8e+01))) false false))))))))

(event OnComponentEndOverlap(OpenCloseCollision)
  (params (OtherActor :type Actor%20Object%20Reference) (OtherComp :type Primitive%20Component%20Object%20Reference) (OtherBodyIndex :type Integer))
  (bind _returnvalue (Transformation|GetActorLocation))
  ;[1 1 1] エネルギー、スタティックメッシュの移動
  (bind _iscastplayer (CallFunction|CheckPlayer OtherActor))
  (if _iscastplayer
    (bind _locationz (Timeline|TimeLine Reverse)
      (:Update
        (Utilities|FlowControl|Sequence
          (:then_0
            (CallFunction|LocationMove (Variables|Default|GetLid) (Variables|SMLocation|GetLidLocation) (* _locationz 0.5)))
          (:then_1
            (CallFunction|LocationMove (Variables|Default|GetPillar) (Variables|SMLocation|GetPillarLocation) (* _locationz 0.5)))
          (:then_2
            (CallFunction|LocationMove (Variables|Default|GetMoveFloor) (Variables|SMLocation|GetFloorLocation) _locationz))
          (:then_3
            (if (Variables|Default|GetIsActive)
              (Transformation|SetActorLocation (Variables|Default|GetEnergy) (Math|Vector|MakeVector (.x _returnvalue) (.y _returnvalue) (+ (.z _returnvalue) (+ _locationz 8e+01))) false false))))))))

(event Custom|DeviceDeactive
  ;[1 0 0] エネルギーが出たらギミックを停止
  (Utilities|FlowControl|Sequence
    (:then_0
      ;[1 1 1] ライトの色を変える
      (Rendering|Material|CreateDynamicMaterialInstance (Variables|Default|GetLight) 0 "/Game/Blueprint/Gimmicks/Material/M_DeviceLight.M_DeviceLight" :!class /Script/Engine.PrimitiveComponent))
    (:then_1
      (for _array_element (Variables|Default|GetGimmick)
        (Utilities|Time|SetTimerbyFunctionName _array_element "SubEnergy" 0.01)))))

(event Custom|DeviceActive
  (bind _light (Variables|Default|GetLight))
  ;[0 1 0] エネルギーが入ったらギミックを起動
  (Utilities|FlowControl|Sequence
    (:then_0
      ;[1 1 1] ライトの色を変える
      (bind _returnvalue (Rendering|Material|CreateDynamicMaterialInstance _light 0 (Rendering|Material|GetMaterial _light 0) :!class /Script/Engine.PrimitiveComponent))
      (Rendering|Material|SetVectorParameterValue _returnvalue "Emissive1" "(R=0.000000,G=1.000000,B=0.000000,A=1.000000)" :!class /Script/Engine.MaterialInstanceDynamic)
      (Rendering|Material|SetVectorParameterValue _returnvalue "Emissive2" "(R=0.100000,G=1.000000,B=0.100000,A=1.000000)" :!class /Script/Engine.MaterialInstanceDynamic))
    (:then_1
      (for _array_element (Variables|Default|GetGimmick)
        (Utilities|Time|SetTimerbyFunctionName _array_element "AddEnergy" 0.01)))))

(fn ConstructionScript
  ;[1 1 1] スタティックメッシュのLocation初期設定
  (Variables|SMLocation|SetFloorLocation (Transformation|GetWorldLocation (Variables|Default|GetMoveFloor)))
  (Variables|SMLocation|SetLidLocation (Transformation|GetWorldLocation (Variables|Default|GetLid)))
  (Variables|SMLocation|SetPillarLocation (Transformation|GetWorldLocation (Variables|Default|GetPillar))))

(fn LocationMove
  (params (StaticMesh :type Static%20Mesh%20Component%20Object%20Reference) (Location :type Vector) (AddLocation :type Float%20%28single-precision%29))
  (bind (_x _y _z) (Math|Vector|BreakVector Location))
  (Transformation|SetWorldLocation StaticMesh (Math|Vector|MakeVector _x _y (+ _z AddLocation)) false false))

(fn CheckPlayer
  (params (Actor :type Object%20Object%20Reference))
  (bind (_asfirst_person_character _bsuccess) (Utilities|Casting|CastToFirstPersonCharacter Actor))
  ;[1 1 1] プレイヤーの判別
  (if _bsuccess
    (if (>= (.z (Transformation|GetActorLocation _asfirst_person_character)) (- (.z (Transformation|GetActorLocation)) 5e+01))
      (if (<= (.z (Transformation|GetActorLocation _asfirst_person_character)) (+ (.z (Transformation|GetActorLocation)) 3.1e+02))
        (Variables|Default|SetIsCastPlayer true)
        (else
          (bind _output_get (Variables|Default|SetIsCastPlayer false :!label _label))))
      (else
        (goto _label)))
    (else
      (goto _label)))
  (return _output_get))