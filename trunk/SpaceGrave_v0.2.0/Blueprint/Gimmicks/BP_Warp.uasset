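; Warp pad gimmick that teleports the player to a paired BP_Warp when stepped into while switched on.
; The construction script links the partner back to this pad, copies IsActive to it and previews ripple material and particles.
; Gimmick_ON/OFF toggle the state and particles, with a timeline fading the ripple's Warp_On parameter.
; Overlap places the player offset from the partner's arrow, redirecting velocity and view along it with a sound.
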(event OnComponentBeginOverlap(Hit_Collision)
  (params (OtherActor :type Actor%20Object%20Reference) (OtherComp :type Primitive%20Component%20Object%20Reference) (OtherBodyIndex :type Integer) (bFromSweep :type Boolean) (SweepResult :type Hit%20Result%20Structure%20%28by%20ref%29))
  (bind (_asfirst_person_character _bsuccess) (Utilities|Casting|CastToFirstPersonCharacter OtherActor))
  (bind _bp_warp (Variables|Default|GetBP_Warp))
  (bind _warp_length (Variables|Default|GetWarp_Length))
  (bind _returnvalue (Transformation|GetActorLocation _bp_warp))
  (bind _point_arrow (Variables|BP_Warp_C|GetPoint_Arrow _bp_warp))
  (bind _returnvalue_2 (Math|Vector|GetForwardVector _point_arrow))
  (bind _returnvalue_3 (* _returnvalue_2 _warp_length))
  ;[1 1 1] ワープ処理
  (if _bsuccess
    (if (Variables|Default|GetIs_Gimmik_On) ; ギミックがOnになってる？
      (Variables|/Script/Engine.MovementComponent|SetVelocity (Variables|/Script/Engine.Character|GetCharacterMovement _asfirst_person_character) _returnvalue_3) ; 残ってるベクトルの向きを変える
      (Pawn|SetControlRotation (Game|GetPlayerController 0) (Transformation|GetWorldRotation _point_arrow)) ; Allowの方を向くように
      (Transformation|SetActorLocation _asfirst_person_character (+ _returnvalue_3 (Math|Vector|MakeVector (.x _returnvalue) (.y _returnvalue) (+ (.z _returnvalue) (Variables|Default|GetWarp_High)))) false false) ; プレイヤーをワープ
      (Audio|PlaySound2D "/Game/Sound/SE/SC_Warp.SC_Warp"))))

(event Custom|Gimmick_ON
  (bind _particlesystem (Variables|Default|GetParticleSystem))
  (bind _sm_warp_ripple (Variables|Default|GetSM_Warp_Ripple))
  ;[1 1 1] 色変化
  (Variables|Default|SetIs_Gimmik_On true)
  (Components|Activation|SetActive _particlesystem true true)
  (Rendering|SetVisibility _particlesystem true false)
  (bind _changetime (Timeline|CalarChange Play)
    (:Update
      (bind _returnvalue (Rendering|Material|CreateDynamicMaterialInstance _sm_warp_ripple 0 (Rendering|Material|GetMaterial _sm_warp_ripple 0) :!class /Script/Engine.PrimitiveComponent))
      (Rendering|Material|SetScalarParameterValue _returnvalue "Warp_On" _changetime :!class /Script/Engine.MaterialInstanceDynamic))))

(event Custom|Gimmick_OFF
  (bind _particlesystem (Variables|Default|GetParticleSystem))
  (bind _sm_warp_ripple (Variables|Default|GetSM_Warp_Ripple))
  ;[1 1 1] 色変化
  (Variables|Default|SetIs_Gimmik_On false)
  (Components|Activation|SetActive _particlesystem false true)
  (Rendering|SetVisibility _particlesystem false false)
  (bind _changetime (Timeline|CalarChange Reverse)
    (:Update
      (bind _returnvalue (Rendering|Material|CreateDynamicMaterialInstance _sm_warp_ripple 0 (Rendering|Material|GetMaterial _sm_warp_ripple 0) :!class /Script/Engine.PrimitiveComponent))
      (Rendering|Material|SetScalarParameterValue _returnvalue "Warp_On" _changetime :!class /Script/Engine.MaterialInstanceDynamic))))

(event EventBeginPlay
  (bind _particlesystem (Variables|Default|GetParticleSystem))
  (bind _sm_warp_ripple (Variables|Default|GetSM_Warp_Ripple))
  ;[1 1 1] 色変化
  (if (Variables|Default|GetIsActive)
    (Variables|Default|SetIs_Gimmik_On true)
    (Components|Activation|SetActive _particlesystem true true)
    (Rendering|SetVisibility _particlesystem true false)
    (bind _changetime (Timeline|CalarChange Play)
      (:Update
        (bind _returnvalue (Rendering|Material|CreateDynamicMaterialInstance _sm_warp_ripple 0 (Rendering|Material|GetMaterial _sm_warp_ripple 0) :!class /Script/Engine.PrimitiveComponent))
        (Rendering|Material|SetScalarParameterValue _returnvalue "Warp_On" _changetime :!class /Script/Engine.MaterialInstanceDynamic)))))

(event EventActorBeginOverlap
  (params (OtherActor :type Actor%20Object%20Reference)))

(event EventTick
  (params (DeltaSeconds :type Float%20%28single-precision%29)))

(fn ConstructionScript
  (bind _particlesystem (Variables|Default|GetParticleSystem))
  (bind _sm_warp_ripple (Variables|Default|GetSM_Warp_Ripple))
  (bind _returnvalue (Rendering|Material|GetMaterial _sm_warp_ripple 0))
  (|CallParentFunction)
  (bind _output_get (Variables|BP_Warp_C|SetBP_Warp (Variables|Default|GetBP_Warp) self))
  (if (Variables|Default|GetIsActive)
    (Variables|/Game/Blueprint/Gimmicks/Blueprint/BP_Gimmick.BP_Gimmick_C|SetIsActive _output_get true)
    (bind _returnvalue_2 (Rendering|Material|CreateDynamicMaterialInstance _sm_warp_ripple 0 _returnvalue :!class /Script/Engine.PrimitiveComponent))
    (Rendering|Material|SetScalarParameterValue _returnvalue_2 "Warp_On" 1.0 :!class /Script/Engine.MaterialInstanceDynamic)
    (Rendering|SetVisibility _particlesystem true false)
    (Components|Activation|SetActive _particlesystem true true)
    (else
      (Variables|/Game/Blueprint/Gimmicks/Blueprint/BP_Gimmick.BP_Gimmick_C|SetIsActive _output_get false)
      (bind _returnvalue_3 (Rendering|Material|CreateDynamicMaterialInstance _sm_warp_ripple 0 _returnvalue :!class /Script/Engine.PrimitiveComponent))
      (Rendering|Material|SetScalarParameterValue _returnvalue_3 "Warp_On" 0.0 :!class /Script/Engine.MaterialInstanceDynamic)
      (Rendering|SetVisibility _particlesystem false false)
      (Components|Activation|SetActive _particlesystem false true))))