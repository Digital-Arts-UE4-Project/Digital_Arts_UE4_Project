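; BP_CableLine is a gimmick actor that builds a segmented cable line from an editable array of rotation, angle and length entries.
; The Construction Script adds a length-scaled mesh per entry and a joint mesh at its rotated end, where the next segment starts.
; At BeginPlay, static mesh children switch from main pass to custom depth rendering, so they show only through effects that read that buffer.
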(event EventBeginPlay
  (for _array_element (Components|GetChildrenComponents (Variables|Default|GetSceneRoot) true)
    (bind _asstatic_mesh_component (Utilities|Casting|CastToStaticMeshComponent _array_element))
    (Class|PrimitiveComponent|SetRenderinMainPass _asstatic_mesh_component false)
    (Rendering|SetRenderCustomDepth _asstatic_mesh_component true)))

(fn ConstructionScript
  (for _array_element (Variables|Default|GetLine)
    ;[1 1 1] RotateとAngleから向きを取得
    (bind _output_get (Variables|Default|SetLineRotate (Math|Rotator|MakeRotator 0.0 (.Rotate (Utilities|Struct|BreakST_CableLine _array_element)) (.Angle (Utilities|Struct|BreakST_CableLine _array_element)))))
    ;[1 1 1] 取得した向きにLineを生成
    (AddComponent|AddStaticMeshComponent false (Math|Transform|MakeTransform (Variables|Default|GetLineLocation) _output_get (Math|Vector|MakeVector (* (.Length (Utilities|Struct|BreakST_CableLine _array_element)) 5.0) 1.0 1.0)))
    ;[1 1 1] 接続部分の生成
    (bind _returnvalue (AddComponent|AddStaticMeshComponent false (Math|Transform|MakeTransform (+ (Math|Vector|RotateVector (Math|Vector|MakeVector (* (.Length (Utilities|Struct|BreakST_CableLine _array_element)) 1e+02) 0.0 0.0) (Variables|Default|GetLineRotate)) (Variables|Default|GetLineLocation)) "0, 0, 0" "1.000000,1,1")))
    (Variables|Default|SetLineLocation (Variables|/Script/Engine.SceneComponent|GetRelativeLocation _returnvalue))))