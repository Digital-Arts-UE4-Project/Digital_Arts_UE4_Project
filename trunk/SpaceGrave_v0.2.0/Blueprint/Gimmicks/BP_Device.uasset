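; Gimmick device that opens as the player character overlaps it and closes when they leave.
; A timeline lifts the lid, pillar and floor, carrying the Energy actor along while the device is active, with a delayed sound.
; InputDevice switches the light material, writes a custom depth stencil value to the device, linked gimmicks and cables, and calls a named function on each gimmick through a short timer.
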(event OnComponentBeginOverlap(OpenCloseCollision)
  (params (OtherActor :type Actor%20Object%20Reference) (OtherComp :type Primitive%20Component%20Object%20Reference) (OtherBodyIndex :type Integer) (bFromSweep :type Boolean) (SweepResult :type Hit%20Result%20Structure%20%28by%20ref%29))
  (bind _returnvalue (Transformation|GetActorLocation))
  ;[1 1 1] エネルギー、スタティックメッシュの移動
  (Utilities|Casting|CastToFirstPersonCharacter OtherActor)
  (CallFunction|PlaySE)
  (bind _locationz (Timeline|TimeLine Play)
    (:Update
      (Utilities|FlowControl|Sequence
        (:then_0
          (CallFunction|LocationMove (Variables|Default|GetLid) (Variables|SMLocation|GetLidLocation) (* _locationz 0.5)))
        (:then_1
          (CallFunction|LocationMove (Variables|Default|GetPillar) (Variables|SMLocation|GetPillarLocation) (* _locationz 0.5)))
        (:then_2
          (CallFunction|LocationMove (Variables|Default|GetMoveFloor) (Variables|SMLocation|GetFloorLocation) _locationz))
        (:then_3
          (if (Variables|Default|GetIsActive)
            (Transformation|SetActorLocation (Variables|Default|GetEnergy) (Math|Vector|MakeVector (.x _returnvalue) (.y _returnvalue) (+ (.z _returnvalue) (+ _locationz 8e+01))) false false)))))))

(event OnComponentEndOverlap(OpenCloseCollision)
  (params (OtherActor :type Actor%20Object%20Reference) (OtherComp :type Primitive%20Component%20Object%20Reference) (OtherBodyIndex :type Integer))
  (bind _returnvalue (Transformation|GetActorLocation))
  ;[1 1 1] エネルギー、スタティックメッシュの移動
  (Utilities|Casting|CastToFirstPersonCharacter OtherActor)
  (CallFunction|PlaySE)
  (bind _locationz (Timeline|TimeLine Reverse)
    (:Update
      (Utilities|FlowControl|Sequence
        (:then_0
          (CallFunction|LocationMove (Variables|Default|GetLid) (Variables|SMLocation|GetLidLocation) (* _locationz 0.5)))
        (:then_1
          (CallFunction|LocationMove (Variables|Default|GetPillar) (Variables|SMLocation|GetPillarLocation) (* _locationz 0.5)))
        (:then_2
          (CallFunction|LocationMove (Variables|Default|GetMoveFloor) (Variables|SMLocation|GetFloorLocation) _locationz))
        (:then_3
          (if (Variables|Default|GetIsActive)
            (Transformation|SetActorLocation (Variables|Default|GetEnergy) (Math|Vector|MakeVector (.x _returnvalue) (.y _returnvalue) (+ (.z _returnvalue) (+ _locationz 8e+01))) false false)))))))

(event Custom|InputDevice
  (params (IsAdd :type Boolean) (DepthValue :type Integer) (FunctionName :type String))
  (bind _light (Variables|Default|GetLight))
  ;[1 1 1] デバイスの起動/停止
  (Variables|Default|SetLocalIsAdd IsAdd)
  (Variables|Default|SetLocalDepthValue DepthValue)
  (Variables|Default|SetLocalFunctionName FunctionName)
  (Utilities|FlowControl|Sequence
    (:then_0
      (if (Variables|Default|GetLocalIsAdd)
        (bind _returnvalue (Rendering|Material|CreateDynamicMaterialInstance _light 0 (Rendering|Material|GetMaterial _light 0) :!class /Script/Engine.PrimitiveComponent))
        (Rendering|Material|SetVectorParameterValue _returnvalue "Emissive1" "(R=0.000000,G=1.000000,B=0.000000,A=1.000000)" :!class /Script/Engine.MaterialInstanceDynamic)
        (Rendering|Material|SetVectorParameterValue _returnvalue "Emissive2" "(R=0.100000,G=1.000000,B=0.100000,A=1.000000)" :!class /Script/Engine.MaterialInstanceDynamic)
        (else
          (Rendering|Material|CreateDynamicMaterialInstance _light 0 "/Game/Blueprint/Gimmicks/Material/M_DeviceLight.M_DeviceLight" :!class /Script/Engine.PrimitiveComponent))))
    (:then_1
      (for _array_element (Components|GetChildrenComponents (Variables|Default|GetDefaultSceneRoot) true)
        (bind _asstatic_mesh_component (Utilities|Casting|CastToStaticMeshComponent _array_element))
        (Rendering|SetCustomDepthStencilValue _asstatic_mesh_component (Variables|Default|GetLocalDepthValue))
        (for _array_element_2 (Variables|Default|GetGimmick)
          (Utilities|FlowControl|Sequence
            (:then_0
              (for _array_element_3 (Components|GetChildrenComponents (Variables|/Game/Blueprint/Gimmicks/Blueprint/BP_Gimmick.BP_Gimmick_C|GetDefaultSceneRoot _array_element_2) true)
                (bind _asstatic_mesh_component_2 (Utilities|Casting|CastToStaticMeshComponent _array_element_3))
                (Rendering|SetCustomDepthStencilValue _asstatic_mesh_component_2 (Variables|Default|GetLocalDepthValue))))
            (:then_1
              (Utilities|Time|SetTimerbyFunctionName _array_element_2 (Variables|Default|GetLocalFunctionName) 0.01))))
        (for _array_element_4 (Variables|Default|GetCableLine)
          (for _array_element_5 (Components|GetChildrenComponents (Variables|/Game/Blueprint/Gimmicks/BP_CableLine.BP_CableLine_C|GetSceneRoot _array_element_4) true)
            (bind _asstatic_mesh_component_3 (Utilities|Casting|CastToStaticMeshComponent _array_element_5))
            (Rendering|SetCustomDepthStencilValue _asstatic_mesh_component_3 (Variables|Default|GetLocalDepthValue))))))))

(event Custom|PlaySE
  ;[1 1 1] エネルギー、スタティックメッシュの移動
  (Utilities|FlowControl|Delay 0.3)
  (Audio|PlaySoundatLocation "/Game/Sound/SE/SC_Device.SC_Device" (Transformation|GetActorLocation)))

(fn ConstructionScript
  ;[1 1 1] スタティックメッシュのLocationの初期設定
  (Variables|SMLocation|SetFloorLocation (Transformation|GetWorldLocation (Variables|Default|GetMoveFloor)))
  (Variables|SMLocation|SetLidLocation (Transformation|GetWorldLocation (Variables|Default|GetLid)))
  (Variables|SMLocation|SetPillarLocation (Transformation|GetWorldLocation (Variables|Default|GetPillar)))
  ;[1 1 1] カスタムデプスの設定
  (for _array_element (Components|GetChildrenComponents (Variables|Default|GetDefaultSceneRoot) true)
    (bind _asstatic_mesh_component (Utilities|Casting|CastToStaticMeshComponent _array_element))
    (Rendering|SetRenderCustomDepth _asstatic_mesh_component true)))

(fn LocationMove
  (params (StaticMesh :type Static%20Mesh%20Component%20Object%20Reference) (Location :type Vector) (AddLocation :type Float%20%28single-precision%29))
  (bind (_x _y _z) (Math|Vector|BreakVector Location))
  (Transformation|SetWorldLocation StaticMesh (Math|Vector|MakeVector _x _y (+ _z AddLocation)) false false))