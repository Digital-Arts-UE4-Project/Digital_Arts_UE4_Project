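; BP_Crystal is a collectible crystal actor that spins in place and flies into the player when picked up.
; BeginPlay plays a timeline that adds yaw rotation to the static mesh.
; GetCrystal captures the player's location once, then a second timeline moves the actor toward that point while scaling the mesh by a curve, destroying the actor when it finishes.
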(event Custom|GetCrystal
  (bind _staticmesh (Variables|Default|GetStaticMesh))
  ;[1 1 1] クリスタル入手
  (bind _output_get (Variables|Default|SetNewVar_0 (Transformation|GetActorLocation (Game|GetPlayerCharacter 0))))
  (bind (_direction _move _scale) (Timeline|Timeline_1 Play)
    (:Update
      (Class|Actor|AddActorWorldTransform (Math|Transform|MakeTransform (* (- _output_get (Transformation|GetActorLocation)) _move) "0, 0, 0" "0, 0, 0") false false)
      (Transformation|SetRelativeScale3D _staticmesh (* (Variables|/Script/Engine.SceneComponent|GetRelativeScale3D _staticmesh) _scale)))
    (:Finished
      (Actor|DestroyActor))))

(event EventBeginPlay
  ;[1 1 1] 回転
  (bind _newtrack_0 (Timeline|Timeline_0 Play)
    (:Update
      (Transformation|AddRelativeRotation (Variables|Default|GetStaticMesh) (Math|Rotator|MakeRotator 0.0 0.0 _newtrack_0) false false))))

(fn ConstructionScript)