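; Spider enemy character that damages the first-person player on contact or when close during a sprint.
; Capsule hits apply damage directly, while Tick sphere-traces around the mesh's spine socket and applies damage every frame the trace hits the player during a sprint.
; BeginSprint and EndSprint switch walk speed and the sprint flag.
; CanSeePlayerPawn sphere-sweeps forward to report whether the player is seen, along with the hit actor.
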(event OnComponentHit(CapsuleComponent)
  (params (OtherActor :type Actor%20Object%20Reference) (OtherComp :type Primitive%20Component%20Object%20Reference) (NormalImpulse :type Vector :default "0, 0, 0") (Hit :type Hit%20Result%20Structure%20%28by%20ref%29))
  (bind _asfirst_person_character (Utilities|Casting|CastToFirstPersonCharacter OtherActor))
  (Game|Damage|ApplyDamage _asfirst_person_character 1.0 0 0))

(event EventBeginPlay
  (Variables|/Script/Engine.CharacterMovementComponent|SetMaxWalkSpeed (Variables|Character|GetCharacterMovement) (Variables|CharaSpec|GetWalkGroundSpeed)))

(event EventTick
  (params (DeltaSeconds :type Float%20%28single-precision%29))
  (bind _mesh (Variables|Character|GetMesh))
  (bind _returnvalue (Transformation|GetSocketLocation _mesh "spine"))
  ;[1 1 1] スプリント時、プレイヤーに近づいたらダメージ
  (if (Variables|Default|GetIsSprint)
    (bind _outhit (Class|KismetSystemLibrary|SphereTraceSingleNEW _returnvalue (+ _returnvalue (Transformation|GetActorForwardVector)) 2.5e+02 "TraceTypeQuery3" false 0 "None" true))
    (bind _asfirst_person_character (Utilities|Casting|CastToFirstPersonCharacter (.HitActor (Collision|BreakHitResult _outhit))))
    (Game|Damage|ApplyDamage _asfirst_person_character 1.0 0 0)))

(fn ConstructionScript)

(fn CanSeePlayerPawn
  (bind _returnvalue (Transformation|GetActorForwardVector))
  (bind _returnvalue_2 (Transformation|GetActorLocation))
  (bind _sightradius (Variables|Trace|GetSightRadius))
  (bind _returnvalue_3 (/ _sightradius 2.0))
  (bind _outhit (Class|KismetSystemLibrary|SphereTraceSingleNEW (+ _returnvalue_2 (* _returnvalue _returnvalue_3)) (+ _returnvalue_2 (* _returnvalue (+ (Variables|Trace|GetSightLength) _returnvalue_3))) (Variables|Trace|GetSightRadius) "TraceTypeQuery3" false 0 "None" true))
  (Utilities|Casting|CastToFirstPersonCharacter (.HitActor (Collision|BreakHitResult _outhit))
    (:then
      (LocalVariables|SetIsPlayer true))
    (:CastFailed
      (LocalVariables|SetIsPlayer false)))
  (return (LocalVariables|GetIsPlayer) (.HitActor (Collision|BreakHitResult _outhit))))

(fn BeginSprint
  (Variables|/Script/Engine.CharacterMovementComponent|SetMaxWalkSpeed (Variables|Character|GetCharacterMovement) (Variables|CharaSpec|GetSprintGroundSpeed))
  (Variables|Default|SetIsSprint true))

(fn EndSprint
  (Variables|/Script/Engine.CharacterMovementComponent|SetMaxWalkSpeed (Variables|Character|GetCharacterMovement) (Variables|CharaSpec|GetWalkGroundSpeed))
  (Variables|Default|SetIsSprint false))