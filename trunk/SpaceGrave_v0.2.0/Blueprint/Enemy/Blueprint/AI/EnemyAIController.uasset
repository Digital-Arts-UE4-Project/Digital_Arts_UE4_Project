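; AI controller for the spider enemy that sets up and runs its patrol behavior.
; On BeginPlay it copies the pawn's patrol points, writes its wait duration to the Blackboard and starts the patrol Behavior Tree.
; Helper functions return the current point and advance the index in a loop.
; A GoToPatrol event, not triggered by BeginPlay, moves between points using AIMoveTo and a self-rescheduling timer.
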(event Custom|GoToPatrol
  (AI|AIMoveTo (Pawn|GetControlledPawn) (CallFunction|GetPatrolLocation) 0 5.0 false
    (:OnSuccess
      (CallFunction|PopPatrolLocation)
      (Utilities|Time|SetTimerbyFunctionName 0 "GoToPatrol" 1.0))))

(event EventBeginPlay
  (bind _asbp_enemy_spider (Utilities|Casting|CastToBP_Enemy_Spider (Pawn|GetControlledPawn)))
  (Variables|Default|SetAI_PatrolPoints (Variables|/Game/Blueprint/Enemy/Blueprint/BP_Enemy_Spider.BP_Enemy_Spider_C|GetPatrolPoints _asbp_enemy_spider))
  (Class|AIController|UseBlackboard "/Game/Blueprint/Enemy/Blueprint/AI/Blackboard_Enemy.Blackboard_Enemy")
  (AI|Components|Blackboard|SetValueasFloat (AI|GetBlackboard 0) (Utilities|Name|MakeLiteralName "PatrolWaitDuration") (Variables|/Game/Blueprint/Enemy/Blueprint/BP_Enemy_Spider.BP_Enemy_Spider_C|GetPatrolWaitDuration _asbp_enemy_spider))
  (AI|RunBehaviorTree "/Game/Blueprint/Enemy/Blueprint/AI/BT_EnemyPatrol.BT_EnemyPatrol"))

(fn ConstructionScript)

(fn GetPatrolLocation
  (return (Transformation|GetActorLocation (Utilities|Array|Get(acopy) (Variables|Default|GetAI_PatrolPoints) (Variables|Default|GetPatrol%20Index)))))

(fn PopPatrolLocation
  (Variables|Default|SetPatrol%20Index (Math|Integer|%(Integer) (+ (Variables|Default|GetPatrol%20Index) 1) (Utilities|Array|Length (Variables|Default|GetAI_PatrolPoints)))))