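; BP_Energy is an energy pickup gimmick that floats and rotates until its physics is switched on.
; A timeline bobs and spins the mesh while physics is off, and PhysicsChenge enables simulation on it.
; Once physical, the first Hit plays a material timeline animating emissive and opacity through a dynamic instance.
; When that finishes, it asks its BP_EnergySpawner to respawn energy and destroys itself.
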(event Custom|PhysicsChenge
  ;[1 1 1] 物理エンジンのOFF
  (Variables|Default|SetIsPhysics true)
  (Physics|SetSimulatePhysics (Variables|Default|GetSM_Energy) true))

(event EventBeginPlay
  (bind _sm_energy (Variables|Default|GetSM_Energy))
  (bind _returnvalue (Transformation|GetRelativeTransform _sm_energy))
  ;[1 1 1] 浮遊
  (bind (_direction _locationz _rotetion) (Timeline|Floating Play)
    (:Update
      (if (not (Variables|Default|GetIsPhysics))
        (Transformation|SetRelativeTransform _sm_energy (Math|Transform|MakeTransform (Math|Vector|MakeVector (.x (.location _returnvalue)) (.y (.location _returnvalue)) (+ (.z (.location _returnvalue)) _locationz)) (Math|Rotator|MakeRotator 0.0 _rotetion _rotetion) (.scale _returnvalue)) false false)))))

(event Collision|EventHit
  (params (MyComp :type Primitive%20Component%20Object%20Reference) (Other :type Actor%20Object%20Reference) (OtherComp :type Primitive%20Component%20Object%20Reference) (bSelfMoved :type Boolean) (HitLocation :type Vector) (HitNormal :type Vector) (NormalImpulse :type Vector) (Hit :type Hit%20Result%20Structure%20%28by%20ref%29))
  (bind _sm_energy (Variables|Default|GetSM_Energy))
  ;[1 1 1] 消去
  (if (Variables|Default|GetIsPhysics)
    (Utilities|FlowControl|DoOnce false
      (:Completed
        (bind _returnvalue (Rendering|Material|CreateDynamicMaterialInstance _sm_energy 0 (Rendering|Material|GetMaterial _sm_energy 0) :!class /Script/Engine.PrimitiveComponent))
        (bind (_direction _emissive _opacity) (Timeline|material Play)
          (:Update
            (Rendering|Material|SetScalarParameterValue _returnvalue "Emissive" _emissive :!class /Script/Engine.MaterialInstanceDynamic)
            (Rendering|Material|SetScalarParameterValue _returnvalue "Opacity" _opacity :!class /Script/Engine.MaterialInstanceDynamic))
          (:Finished
            (Default|RespawnEnergy (.AsBP%20Energy%20Spawner (Utilities|Casting|CastToBP_EnergySpawner (Variables|Default|GetSpawner))))
            (Actor|DestroyActor)))))))

(fn ConstructionScript)