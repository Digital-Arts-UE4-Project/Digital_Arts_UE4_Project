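; Flamethrower gimmick that emits fire along its Arrow component and can be switched on and off.
; On BeginPlay it spawns a BP_Fire slightly above itself, using the Arrow's rotation with a pitch offset, then activates or deactivates that actor's PMFire component according to IsActive.
; GimmickON and GimmickOFF events later toggle the same PMFire component on the spawned fire, without respawning it.
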(event EventGimmickOFF
  ;[1 1 1] ギミックのON/OFF
  (Components|Activation|Deactivate (Variables|/Game/MainAsset/Blueprints/Gimmicks/Blueprint/BP_Fire.BP_Fire_C|GetPM_Fire (stale EventBeginPlay _returnvalue_3))))

(event EventBeginPlay
  (bind _returnvalue (Transformation|GetActorTransform))
  (bind _arrow (Variables|Default|GetArrow))
  (bind (_location _rotation _scale) (Math|Transform|BreakTransform _returnvalue))
  (bind _returnvalue_2 (Transformation|GetWorldRotation _arrow))
  ;[1 1 1] 炎の初期表示
  (bind _returnvalue_3 (Game|SpawnActorfromClass "/Game/MainAsset/Blueprints/Gimmicks/Blueprint/BP_Fire.BP_Fire_C" (Math|Transform|MakeTransform (Math|Vector|MakeVector (.x _location) (.y _location) (+ (.z _location) 5e+01)) (Math|Rotator|MakeRotator (.roll _returnvalue_2) (+ (.pitch _returnvalue_2) -9e+01) (.yaw _returnvalue_2)) _scale) "Undefined" 0 0))
  (if (Variables|Default|GetIsActive)
    (Components|Activation|Activate (Variables|/Game/MainAsset/Blueprints/Gimmicks/Blueprint/BP_Fire.BP_Fire_C|GetPM_Fire _returnvalue_3) false)
    (else
      (Components|Activation|Deactivate (Variables|/Game/MainAsset/Blueprints/Gimmicks/Blueprint/BP_Fire.BP_Fire_C|GetPM_Fire _returnvalue_3)))))

(event EventGimmickON
  ;[1 1 1] ギミックのON/OFF
  (Components|Activation|Activate (Variables|/Game/MainAsset/Blueprints/Gimmicks/Blueprint/BP_Fire.BP_Fire_C|GetPM_Fire (stale EventBeginPlay _returnvalue_3)) false))

(fn ConstructionScript)