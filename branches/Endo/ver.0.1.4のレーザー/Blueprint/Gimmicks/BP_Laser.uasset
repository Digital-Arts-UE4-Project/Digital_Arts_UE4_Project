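; BP_Laser is a laser fence gimmick: two poles with horizontal laser lines between them, switchable on and off.
; On BeginPlay it positions and scales the poles from Width and Height, then spawns LaserCount evenly stacked BP_LaserLine actors scaled to the width.
; The spawned lines are kept in LaserArrey, and IsActive sets their initial particle state.
; GimmickON and GimmickOFF activate or deactivate every line's particle system.
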(event EventGimmickON
  (bind _laserarrey (Variables|Default|GetLaserArrey))
  ;[1 1 1] ギミックのON/OFF
  (for _index (range 0 (Utilities|Array|LastIndex _laserarrey))
    (Components|Activation|Activate (Variables|/Game/Blueprint/Gimmicks/Blueprint/BP_LaserLine.BP_LaserLine_C|GetParticleSystem (Utilities|Array|Get(acopy) _laserarrey _index)) false)))

(event EventGimmickOFF
  (bind _laserarrey (Variables|Default|GetLaserArrey))
  ;[1 1 1] ギミックのON/OFF
  (for _index (range 0 (Utilities|Array|LastIndex _laserarrey))
    (Components|Activation|Deactivate (Variables|/Game/Blueprint/Gimmicks/Blueprint/BP_LaserLine.BP_LaserLine_C|GetParticleSystem (Utilities|Array|Get(acopy) _laserarrey _index)))))

(event EventBeginPlay
  (bind _returnvalue (Transformation|GetActorTransform))
  (bind _sm_leftpole (Variables|Default|GetSM_LeftPole))
  (bind _sm_rightpole (Variables|Default|GetSM_RightPole))
  (bind _laserarrey (Variables|Default|GetLaserArrey))
  (bind _height (Variables|Default|GetHeight))
  (bind _height_2 (Variables|Default|GetHeight))
  (bind _returnvalue_2 (Utilities|Array|LastIndex _laserarrey))
  (bind _returnvalue_3 (Transformation|GetRelativeTransform _sm_rightpole))
  (bind _returnvalue_4 (Transformation|GetRelativeTransform _sm_leftpole))
  ;[1 1 1] 初期設定
  (Transformation|SetRelativeTransform _sm_leftpole (Math|Transform|MakeTransform (Math|Vector|MakeVector (+ (* (Variables|Default|GetWidth) 5e+01) -5.0) (.y (.location _returnvalue_4)) (+ (.z (.location _returnvalue_4)) (* 5e+01 (- _height_2 1.0)))) (.rotation _returnvalue_4) (Math|Vector|MakeVector (.x (.scale _returnvalue_4)) (.y (.scale _returnvalue_4)) _height_2)) false false)
  (Transformation|SetRelativeTransform _sm_rightpole (Math|Transform|MakeTransform (Math|Vector|MakeVector (+ (* (Variables|Default|GetWidth) -5e+01) 5.0) (.y (.location _returnvalue_3)) (+ (.z (.location _returnvalue_3)) (* 5e+01 (- _height 1.0)))) (.rotation _returnvalue_3) (Math|Vector|MakeVector (.x (.scale _returnvalue_3)) (.y (.scale _returnvalue_3)) _height)) false false)
  (for _index (range 1 (Math|Float|Truncate (Variables|Default|GetLaserCount)))
    (bind _returnvalue_5 (Game|SpawnActorfromClass "/Game/Blueprint/Gimmicks/Blueprint/BP_LaserLine.BP_LaserLine_C" (Math|Transform|MakeTransform (Math|Vector|MakeVector (.x (.location _returnvalue)) (.y (.location _returnvalue)) (+ (* (Math|Conversions|ToFloat(Integer) _index) (/ (* (Variables|Default|GetHeight) 1e+02) (Variables|Default|GetLaserCount))) (.z (.location _returnvalue)) -2.0)) (.rotation _returnvalue) (Math|Vector|MakeVector (/ (Variables|Default|GetWidth) 4.0) (.y (.scale _returnvalue)) (.z (.scale _returnvalue)))) "Undefined" 0 0))
    (Utilities|Array|Add (Variables|Default|GetLaserArrey) _returnvalue_5))
  (if (Variables|Default|GetIsActive)
    (for _index_2 (range 0 _returnvalue_2)
      (Components|Activation|Activate (Variables|/Game/Blueprint/Gimmicks/Blueprint/BP_LaserLine.BP_LaserLine_C|GetParticleSystem (Utilities|Array|Get(acopy) _laserarrey _index_2)) false))
    (else
      (for _index_3 (range 0 _returnvalue_2)
        (Components|Activation|Deactivate (Variables|/Game/Blueprint/Gimmicks/Blueprint/BP_LaserLine.BP_LaserLine_C|GetParticleSystem (Utilities|Array|Get(acopy) _laserarrey _index_3)))))))

(fn ConstructionScript)