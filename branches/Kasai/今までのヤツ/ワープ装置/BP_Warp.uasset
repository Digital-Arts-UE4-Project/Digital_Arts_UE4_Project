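; BP_Warp is a warp-pad gimmick that teleports the first-person player to a linked BP_Warp.
; Gimmick_ON/OFF, or IsActive at BeginPlay, toggle the warp and play or reverse a timeline, whose forward updates feed the ripple material's Warp_On parameter.
; While on, overlap moves the player above and ahead of the partner, matching control rotation to its PointArrow.
; The construction script back-links the partner to itself, making pairs two-way.
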(event OnComponentBeginOverlap(Hit_Collision)
  (params (OtherActor :type Actor%20Object%20Reference) (OtherComp :type Primitive%20Component%20Object%20Reference) (OtherBodyIndex :type Integer) (bFromSweep :type Boolean) (SweepResult :type Hit%20Result%20Structure%20%28by%20ref%29))
  (bind (_asfirst_person_character _bsuccess) (Utilities|Casting|CastToFirstPersonCharacter OtherActor))
  (bind _bp_warp (Variables|Default|GetBP_Warp))
  (bind _returnvalue (Transformation|GetActorLocation _bp_warp))
  (bind _point_arrow (Variables|BP_Warp_C|GetPoint_Arrow _bp_warp))
  ;[1 1 1] ワープ処理
  (if _bsuccess
    (if (Variables|Default|GetIs_Gimmik_On) ; ギミックがOnになってる？
      (Transformation|SetActorLocation _asfirst_person_character (+ (Math|Vector|MakeVector (.x _returnvalue) (.y _returnvalue) (+ (.z _returnvalue) 2e+02)) (* (Math|Vector|GetForwardVector _point_arrow) 3e+02)) false false) ; プレイヤーをワープ
      (Pawn|SetControlRotation (Game|GetPlayerController 0) (Transformation|GetWorldRotation _point_arrow)) ; 常にAllowの方を向くように
    )))

(event Custom|Gimmick_ON
  (bind _sm_warp_ripple (Variables|Default|GetSM_Warp_Ripple))
  ;[1 1 1] 色変化
  (Variables|Default|SetIs_Gimmik_On true)
  (bind _changetime (Timeline|CalarChange Play)
    (:Update
      (bind _returnvalue (Rendering|Material|CreateDynamicMaterialInstance _sm_warp_ripple 0 (Rendering|Material|GetMaterial _sm_warp_ripple 0) :!class /Script/Engine.PrimitiveComponent))
      (Rendering|Material|SetScalarParameterValue _returnvalue "Warp_On" _changetime :!class /Script/Engine.MaterialInstanceDynamic))))

(event Custom|Gimmick_OFF
  (bind _sm_warp_ripple (Variables|Default|GetSM_Warp_Ripple))
  ;[1 1 1] 色変化
  (Variables|Default|SetIs_Gimmik_On false)
  (bind _changetime (Timeline|CalarChange Reverse)
    (:Update
      (bind _returnvalue (Rendering|Material|CreateDynamicMaterialInstance _sm_warp_ripple 0 (Rendering|Material|GetMaterial _sm_warp_ripple 0) :!class /Script/Engine.PrimitiveComponent))
      (Rendering|Material|SetScalarParameterValue _returnvalue "Warp_On" _changetime :!class /Script/Engine.MaterialInstanceDynamic))))

(event EventBeginPlay
  (bind _sm_warp_ripple (Variables|Default|GetSM_Warp_Ripple))
  ;[1 1 1] 色変化
  (if (Variables|Default|GetIsActive)
    (Variables|Default|SetIs_Gimmik_On true)
    (bind _changetime (Timeline|CalarChange Play)
      (:Update
        (bind _returnvalue (Rendering|Material|CreateDynamicMaterialInstance _sm_warp_ripple 0 (Rendering|Material|GetMaterial _sm_warp_ripple 0) :!class /Script/Engine.PrimitiveComponent))
        (Rendering|Material|SetScalarParameterValue _returnvalue "Warp_On" _changetime :!class /Script/Engine.MaterialInstanceDynamic)))))

(event EventActorBeginOverlap
  (params (OtherActor :type Actor%20Object%20Reference)))

(event EventTick
  (params (DeltaSeconds :type Float%20%28single-precision%29)))

(fn ConstructionScript
  (|CallParentFunction)
  (Variables|BP_Warp_C|SetBP_Warp (Variables|Default|GetBP_Warp) self))