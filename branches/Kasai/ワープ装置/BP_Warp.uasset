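; Warp pad gimmick that teleports the player to its linked BP_Warp, which the construction script points back at this pad to form a two-way pair.
; IsActive at BeginPlay or GimmickON/OFF events set the on state and drive a timeline animating the ripple material's Warp_On parameter.
; After an overlap and short delay, Check_On_Player confirms FirstPersonCharacter2 is still over the pad, then, if on, moves it above the partner.
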(event OnComponentBeginOverlap(Hit_Collision)
  (params (OtherActor :type Actor%20Object%20Reference) (OtherComp :type Primitive%20Component%20Object%20Reference) (OtherBodyIndex :type Integer) (bFromSweep :type Boolean) (SweepResult :type Hit%20Result%20Structure%20%28by%20ref%29))
  (bind _bp_warp (Variables|Default|GetBP_Warp))
  (bind _returnvalue (Transformation|GetActorLocation _bp_warp))
  ;[1 1 1] ワープ処理
  (Utilities|FlowControl|Delay 1.5) ; ワープ開始までの時間
  (bind (_output_get _outputpin) (|Check_On_Player OtherActor)) ; 装置の上に乗ってるか確認
  (if _output_get
    (if (Variables|Default|GetIs_Gimmik_On) ; ギミックがOnになってる？
      (Transformation|SetActorLocation _outputpin (Math|Vector|MakeVector (.x _returnvalue) (.y _returnvalue) (+ (.z _returnvalue) (Variables|Default|GetWarp_High))) false false))))

(event EventGimmickON
  (bind _sm_warp_ripple (Variables|Default|GetSM_Warp_Ripple))
  ;[1 1 1] 色変化
  (Variables|Default|SetIs_Gimmik_On true)
  (bind _changetime (Timeline|CalarChange Play)
    (:Update
      (bind _returnvalue (Rendering|Material|CreateDynamicMaterialInstance _sm_warp_ripple 0 (Rendering|Material|GetMaterial _sm_warp_ripple 0) :!class /Script/Engine.PrimitiveComponent))
      (Rendering|Material|SetScalarParameterValue _returnvalue "Warp_On" _changetime :!class /Script/Engine.MaterialInstanceDynamic))))

(event EventGimmickOFF
  (bind _sm_warp_ripple (Variables|Default|GetSM_Warp_Ripple))
  ;[1 1 1] 色変化
  (Variables|Default|SetIs_Gimmik_On false)
  (bind _changetime (Timeline|CalarChange Reverse)
    (:Update
      (bind _returnvalue (Rendering|Material|CreateDynamicMaterialInstance _sm_warp_ripple 0 (Rendering|Material|GetMaterial _sm_warp_ripple 0) :!class /Script/Engine.PrimitiveComponent))
      (Rendering|Material|SetScalarParameterValue _returnvalue "Warp_On" _changetime :!class /Script/Engine.MaterialInstanceDynamic))))

(event EventBeginPlay
  (bind _sm_warp_ripple (Variables|Default|GetSM_Warp_Ripple))
  ;[1 1 1] 色変化
  (if (Variables|Default|GetIsActive)
    (Variables|Default|SetIs_Gimmik_On true)
    (bind _changetime (Timeline|CalarChange Play)
      (:Update
        (bind _returnvalue (Rendering|Material|CreateDynamicMaterialInstance _sm_warp_ripple 0 (Rendering|Material|GetMaterial _sm_warp_ripple 0) :!class /Script/Engine.PrimitiveComponent))
        (Rendering|Material|SetScalarParameterValue _returnvalue "Warp_On" _changetime :!class /Script/Engine.MaterialInstanceDynamic)))))

(event EventActorBeginOverlap
  (params (OtherActor :type Actor%20Object%20Reference)))

(event EventTick
  (params (DeltaSeconds :type Float%20%28single-precision%29)))

(fn ConstructionScript
  (|CallParentFunction)
  (Variables|BP_Warp_C|SetBP_Warp (Variables|Default|GetBP_Warp) self))