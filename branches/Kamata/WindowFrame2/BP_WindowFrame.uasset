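; BP_WindowFrame is a window frame of four pieces (left, right, up, down) that resizes from FrameWidth and FrameHigh.
; The construction script feeds each piece's relative transform through a shared Frame function, changing only X/Z location and scale.
; Width stretches the top and bottom and height stretches the sides, with math expressions adding offsets to side scale and to right and top positions.
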(fn ConstructionScript
  (bind _rightframe (Variables|Default|GetRightFrame))
  (bind _framehigh (Variables|Default|GetFrameHigh))
  (bind _framehigh_2 (Variables|Default|GetFrameHigh))
  (bind _framewidth (Variables|Default|GetFrameWidth))
  (bind _framewidth_2 (Variables|Default|GetFrameWidth))
  (bind _leftframe (Variables|Default|GetLeftFrame))
  (bind _downframe (Variables|Default|GetDownFrame))
  (bind _upframe (Variables|Default|GetUpFrame))
  (bind _returnvalue (Transformation|GetRelativeTransform _leftframe))
  (bind _returnvalue_2 (Transformation|GetRelativeTransform _rightframe))
  (bind _returnvalue_3 (Transformation|GetRelativeTransform _upframe))
  (bind _returnvalue_4 (Transformation|GetRelativeTransform _downframe))
  ;[1 1 1] 左のフレーム
  (CallFunction|Frame _leftframe (.x (.location _returnvalue)) (* (.z (.location _returnvalue)) _framehigh) (.x (.scale _returnvalue)) (|((Sz*h)+((h-1)*0.250000)) (.z (.scale _returnvalue)) _framehigh))
  ;[1 1 1] 右のフレーム
  (CallFunction|Frame _rightframe (|((Lx*w)+((w-1)*5)) (Variables|Default|GetFrameWidth) (.x (.location _returnvalue_2))) (* (.z (.location _returnvalue_2)) _framehigh_2) (.x (.scale _returnvalue_2)) (|((Sz*h)+((h-1)*0.250000)) (.z (.scale _returnvalue_2)) _framehigh_2))
  ;[1 1 1] 下のフレーム
  (CallFunction|Frame _downframe (* (.x (.location _returnvalue_4)) _framewidth) (.z (.location _returnvalue_4)) (* (.x (.scale _returnvalue_4)) _framewidth) (.z (.scale _returnvalue_4)))
  ;[1 1 1] 上のフレーム
  (CallFunction|Frame _upframe (* (.x (.location _returnvalue_3)) _framewidth_2) (|((Lz*h)+((h-1)*5)) (.z (.location _returnvalue_3)) (Variables|Default|GetFrameHigh)) (* _framewidth_2 (.x (.scale _returnvalue_3))) (.z (.scale _returnvalue_3))))

(fn Frame
  (params (FrameType :type Static%20Mesh%20Component%20Object%20Reference) (Location%20X :type Float%20%28single-precision%29) (Location%20Z :type Float%20%28single-precision%29) (Scale%20X :type Float%20%28single-precision%29) (Scale%20Z :type Float%20%28single-precision%29))
  (bind _returnvalue (Transformation|GetRelativeTransform FrameType))
  ;[1 1 1] フレームのX、Zの座標、大きさを変える
  (Transformation|SetRelativeTransform FrameType (Math|Transform|MakeTransform (Math|Vector|MakeVector Location%20X (.y (.location _returnvalue)) Location%20Z) (.rotation _returnvalue) (Math|Vector|MakeVector Scale%20X (.y (.scale _returnvalue)) Scale%20Z)) false false))