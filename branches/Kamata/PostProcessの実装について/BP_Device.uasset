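; Energy-powered device that switches linked gimmicks on or off and opens when the player approaches within its height range.
; Overlap plays or reverses a timeline raising the lid, pillar and floor, carrying the Energy actor while active.
; DeviceActive and DeviceDeactive change the light and call AddEnergy or SubEnergy on gimmicks by timer.
; CustomDepthEdit sets stencil values on device, gimmick and cable meshes for green/red post-process coloring.
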(event OnComponentBeginOverlap(OpenCloseCollision)
  (params (OtherActor :type Actor%20Object%20Reference) (OtherComp :type Primitive%20Component%20Object%20Reference) (OtherBodyIndex :type Integer) (bFromSweep :type Boolean) (SweepResult :type Hit%20Result%20Structure%20%28by%20ref%29))
  (bind _returnvalue (Transformation|GetActorLocation))
  ;[1 1 1] エネルギー、スタティックメッシュの移動
  (bind _iscastplayer (CallFunction|CheckPlayer OtherActor))
  (if _iscastplayer
    (bind _locationz (Timeline|TimeLine Play)
      (:Update
        (Utilities|FlowControl|Sequence
          (:then_0
            (CallFunction|LocationMove (Variables|Default|GetLid) (Variables|SMLocation|GetLidLocation) (* _locationz 0.5)))
          (:then_1
            (CallFunction|LocationMove (Variables|Default|GetPillar) (Variables|SMLocation|GetPillarLocation) (* _locationz 0.5)))
          (:then_2
            (CallFunction|LocationMove (Variables|Default|GetMoveFloor) (Variables|SMLocation|GetFloorLocation) _locationz))
          (:then_3
            (if (Variables|Default|GetIsActive)
              (Transformation|SetActorLocation (Variables|Default|GetEnergy) (Math|Vector|MakeVector (.x _returnvalue) (.y _returnvalue) (+ (.z _returnvalue) (+ _locationz 8e+01))) false false))))))))

(event OnComponentEndOverlap(OpenCloseCollision)
  (params (OtherActor :type Actor%20Object%20Reference) (OtherComp :type Primitive%20Component%20Object%20Reference) (OtherBodyIndex :type Integer))
  (bind _returnvalue (Transformation|GetActorLocation))
  ;[1 1 1] エネルギー、スタティックメッシュの移動
  (bind _iscastplayer (CallFunction|CheckPlayer OtherActor))
  (if _iscastplayer
    (bind _locationz (Timeline|TimeLine Reverse)
      (:Update
        (Utilities|FlowControl|Sequence
          (:then_0
            (CallFunction|LocationMove (Variables|Default|GetLid) (Variables|SMLocation|GetLidLocation) (* _locationz 0.5)))
          (:then_1
            (CallFunction|LocationMove (Variables|Default|GetPillar) (Variables|SMLocation|GetPillarLocation) (* _locationz 0.5)))
          (:then_2
            (CallFunction|LocationMove (Variables|Default|GetMoveFloor) (Variables|SMLocation|GetFloorLocation) _locationz))
          (:then_3
            (if (Variables|Default|GetIsActive)
              (Transformation|SetActorLocation (Variables|Default|GetEnergy) (Math|Vector|MakeVector (.x _returnvalue) (.y _returnvalue) (+ (.z _returnvalue) (+ _locationz 8e+01))) false false))))))))

(event Custom|DeviceDeactive
  ;[1 0 0] エネルギーが出たらギミックを停止
  (Utilities|FlowControl|Sequence
    (:then_0
      ;[1 1 1] ライトの色を変える
      (Rendering|Material|CreateDynamicMaterialInstance (Variables|Default|GetLight) 0 "/Game/Blueprint/Gimmicks/Material/M_DeviceLight.M_DeviceLight" :!class /Script/Engine.PrimitiveComponent))
    (:then_1
      (for _array_element (Variables|Default|GetGimmick)
        (Utilities|Time|SetTimerbyFunctionName _array_element "SubEnergy" 0.01)
        ;[1 0 0] ポストプロセスでの色を赤にする
        (CallFunction|CustomDepthEdit _array_element false) ; ギミックの色を赤にする
      )
      (for _array_element_2 (Variables|Default|GetCableLine)
        (CallFunction|CustomDepthEdit _array_element_2 false) ; ラインの色を赤にする
      )
      (CallFunction|CustomDepthEdit self false) ; 装置の色を赤にする
    )))

(event Custom|DeviceActive
  (bind _light (Variables|Default|GetLight))
  ;[0 1 0] エネルギーが入ったらギミックを起動
  (Utilities|FlowControl|Sequence
    (:then_0
      ;[1 1 1] ライトの色を変える
      (bind _returnvalue (Rendering|Material|CreateDynamicMaterialInstance _light 0 (Rendering|Material|GetMaterial _light 0) :!class /Script/Engine.PrimitiveComponent))
      (Rendering|Material|SetVectorParameterValue _returnvalue "Emissive1" "(R=0.000000,G=1.000000,B=0.000000,A=1.000000)" :!class /Script/Engine.MaterialInstanceDynamic)
      (Rendering|Material|SetVectorParameterValue _returnvalue "Emissive2" "(R=0.100000,G=1.000000,B=0.100000,A=1.000000)" :!class /Script/Engine.MaterialInstanceDynamic))
    (:then_1
      (for _array_element (Variables|Default|GetGimmick)
        (Utilities|Time|SetTimerbyFunctionName _array_element "AddEnergy" 0.01)
        ;[0 1 0] ポストプロセスでの色を緑にする
        (CallFunction|CustomDepthEdit _array_element true) ; ギミックの色を緑にする
      )
      (for _array_element_2 (Variables|Default|GetCableLine)
        (CallFunction|CustomDepthEdit _array_element_2 true) ; ラインの色を緑にする
      )
      (CallFunction|CustomDepthEdit self true) ; 装置の色を緑にする
    )))

(event EventBeginPlay
  ;[1 1 1] ギミックと装置にCustomDepthを入れる
  (for _array_element (Variables|Default|GetGimmick)
    (CallFunction|CustomDepthEdit _array_element false))
  (CallFunction|CustomDepthEdit self false))

(fn ConstructionScript
  ;[1 1 1] スタティックメッシュのLocation初期設定
  (Variables|SMLocation|SetFloorLocation (Transformation|GetWorldLocation (Variables|Default|GetMoveFloor)))
  (Variables|SMLocation|SetLidLocation (Transformation|GetWorldLocation (Variables|Default|GetLid)))
  (Variables|SMLocation|SetPillarLocation (Transformation|GetWorldLocation (Variables|Default|GetPillar))))

(fn LocationMove
  (params (StaticMesh :type Static%20Mesh%20Component%20Object%20Reference) (Location :type Vector) (AddLocation :type Float%20%28single-precision%29))
  (bind (_x _y _z) (Math|Vector|BreakVector Location))
  (Transformation|SetWorldLocation StaticMesh (Math|Vector|MakeVector _x _y (+ _z AddLocation)) false false))

(fn CheckPlayer
  (params (Actor :type Object%20Object%20Reference))
  (bind (_asfirst_person_character _bsuccess) (Utilities|Casting|CastToFirstPersonCharacter Actor))
  ;[1 1 1] プレイヤーの判別
  (if _bsuccess
    (if (>= (.z (Transformation|GetActorLocation _asfirst_person_character)) (- (.z (Transformation|GetActorLocation)) 5e+01))
      (if (<= (.z (Transformation|GetActorLocation _asfirst_person_character)) (+ (.z (Transformation|GetActorLocation)) 3.1e+02))
        (Variables|Default|SetIsCastPlayer true)
        (else
          (bind _output_get (Variables|Default|SetIsCastPlayer false :!label _label))))
      (else
        (goto _label)))
    (else
      (goto _label)))
  (return _output_get))

(fn CustomDepthEdit
  (params (CustomDepthTarget :type Actor%20Object%20Reference) (ON :type Boolean))
  (Utilities|FlowControl|Sequence
    (:then_0
      ;[1 1 1] ラインのStaticMeshを取得する
      (bind _asbp_cable_line (Utilities|Casting|CastToBP_CableLine CustomDepthTarget))
      (for _array_element (Components|GetChildrenComponents (Variables|/Game/CableLine/BP_CableLine.BP_CableLine_C|GetScene _asbp_cable_line) true)
        (bind _asstatic_mesh_component (Utilities|Casting|CastToStaticMeshComponent _array_element))
        ;[1 1 1] CustomDepthに値が入っていなければ値を入れる
        (Variables|Default|SetTargetStaticMesh _asstatic_mesh_component)
        (if (Variables|/Script/Engine.PrimitiveComponent|GetbRenderCustomDepth _asstatic_mesh_component)
          ;[1 1 1] ONにチェックが入っていれば緑、入っていなければ赤色にする
          (if ON
            (Rendering|SetCustomDepthStencilValue (Variables|Default|GetTargetStaticMesh) 1)
            (else
              (Rendering|SetCustomDepthStencilValue (Variables|Default|GetTargetStaticMesh) 0)))
          (else
            (Rendering|SetRenderCustomDepth (Variables|Default|GetTargetStaticMesh) true)))))
    (:then_1
      ;[1 1 1] ギミックのStaticMeshを取得する
      (bind _asbp_gimmick (Utilities|Casting|CastToBP_Gimmick CustomDepthTarget))
      (for _array_element_2 (Components|GetChildrenComponents (Variables|/Game/Blueprint/Gimmicks/Blueprint/BP_Gimmick.BP_Gimmick_C|GetDefaultSceneRoot _asbp_gimmick) true)
        (bind _asstatic_mesh_component_2 (Utilities|Casting|CastToStaticMeshComponent _array_element_2))
        (Variables|Default|SetTargetStaticMesh _asstatic_mesh_component_2)
        (if (Variables|/Script/Engine.PrimitiveComponent|GetbRenderCustomDepth _asstatic_mesh_component_2)
          (if ON
            (Rendering|SetCustomDepthStencilValue (Variables|Default|GetTargetStaticMesh) 1)
            (else
              (Rendering|SetCustomDepthStencilValue (Variables|Default|GetTargetStaticMesh) 0)))
          (else
            (Rendering|SetRenderCustomDepth (Variables|Default|GetTargetStaticMesh) true)))))
    (:then_2
      ;[1 1 1] 装置のStaticMeshを取得する
      (bind _asbp_device (Utilities|Casting|CastToBP_Device CustomDepthTarget))
      (for _array_element_3 (Components|GetChildrenComponents (Variables|BP_Device_C|GetDefaultSceneRoot _asbp_device) true)
        (bind _asstatic_mesh_component_3 (Utilities|Casting|CastToStaticMeshComponent _array_element_3))
        (Variables|Default|SetTargetStaticMesh _asstatic_mesh_component_3)
        (if (Variables|/Script/Engine.PrimitiveComponent|GetbRenderCustomDepth _asstatic_mesh_component_3)
          (if ON
            (Rendering|SetCustomDepthStencilValue (Variables|Default|GetTargetStaticMesh) 1)
            (else
              (Rendering|SetCustomDepthStencilValue (Variables|Default|GetTargetStaticMesh) 0)))
          (else
            (Rendering|SetRenderCustomDepth (Variables|Default|GetTargetStaticMesh) true)))))))