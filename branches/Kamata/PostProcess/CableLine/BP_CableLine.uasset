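; BP_CableLine is a post-process cable line actor that builds a segmented cable path from static meshes.
; The construction script chains segments from the Line array, orienting each by Rotate and Angle and stretching it by Length.
; A curve mesh joins consecutive segments at the computed endpoint, which becomes the next segment's origin.
; BeginPlay disables main-pass rendering on the collected SMCableLine meshes, hiding the cable during play.
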(event EventBeginPlay
  ;[1 1 1] プレイ中は見えなくなる
  (Class|PrimitiveComponent|SetRenderinMainPass (Variables|ColorChange|GetSM_CableLine) false))

(fn ConstructionScript
  (bind _line (Variables|LineCreate|GetLine))
  (bind _returnvalue (Utilities|Array|LastIndex _line))
  (for _index (range 0 _returnvalue)
    ;[1 1 1] RotateとAngleから向きを取得する
    (bind _output_get (Variables|LineCreate|SetLineRotate (Math|Rotator|MakeRotator (.Rotate (Utilities|Struct|BreakST_CableLine (Utilities|Array|Get(acopy) (Variables|LineCreate|GetLine) _index))) (.Angle (Utilities|Struct|BreakST_CableLine (Utilities|Array|Get(acopy) (Variables|LineCreate|GetLine) _index))) (.Rotate (Utilities|Struct|BreakST_CableLine (Utilities|Array|Get(acopy) (Variables|LineCreate|GetLine) _index))))))
    ;[1 1 1] 取得した向きにLineを作る
    (bind _returnvalue_2 (AddComponent|AddStaticMeshComponent false (Math|Transform|MakeTransform (Variables|LineCreate|GetLineLocation) _output_get (Math|Vector|MakeVector (* (.Length (Utilities|Struct|BreakST_CableLine (Utilities|Array|Get(acopy) (Variables|LineCreate|GetLine) _index))) 5.0) 1.0 1.0))))
    ;[1 1 1] 見えなくする部分を配列に加える
    (Utilities|Array|Add (Variables|ColorChange|GetSM_CableLine) _returnvalue_2)
    (if (< _index _returnvalue) ; 最後はカーブを作らない
      ;[1 1 1] カーブを作る
      (bind _returnvalue_3 (AddComponent|AddStaticMeshComponent false (Math|Transform|MakeTransform (+ (Math|Vector|RotateVector (Math|Vector|MakeVector (* (.Length (Utilities|Struct|BreakST_CableLine (Utilities|Array|Get(acopy) (Variables|LineCreate|GetLine) _index))) 1e+02) 0.0 0.0) (Variables|LineCreate|GetLineRotate)) (Variables|LineCreate|GetLineLocation)) "0, 0, 0" "1.000000,1,1")))
      (Variables|LineCreate|SetLineLocation (Variables|/Script/Engine.SceneComponent|GetRelativeLocation _returnvalue_3))
      ;[1 1 1] 見えなくなる部分を配列に加える
      (Utilities|Array|Add (Variables|ColorChange|GetSM_CableLine) _returnvalue_3))))