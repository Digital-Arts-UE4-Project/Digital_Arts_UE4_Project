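; BP_Lift is a lift platform that shuttles back and forth along its local X axis while IsActive is set.
; BeginPlay positions both end meshes and scales the laser meshes from Length, so the layout applies only at runtime.
; Tick moves the platform by Speed until near an end, where a DoOnce-gated timeline adds per-update MoveEnd offsets.
; After WaitTime, it flips Reverse and resets that gate and timeline.
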(event EventBeginPlay
  (bind _length (Variables|Default|GetLength))
  (bind _sm_liftend1 (Variables|Default|GetSM_LiftEnd1))
  (bind _sm_liftend2 (Variables|Default|GetSM_LiftEnd2))
  (bind _length_2 (Variables|Default|GetLength))
  (bind _returnvalue (/ _length 2.0))
  (bind _returnvalue_2 (* _length_2 1e+02))
  (bind _relativelocation (Variables|/Script/Engine.SceneComponent|GetRelativeLocation _sm_liftend2))
  (bind _relativelocation_2 (Variables|/Script/Engine.SceneComponent|GetRelativeLocation _sm_liftend1))
  (bind _returnvalue_3 (- _returnvalue 0.1))
  (bind _returnvalue_4 (+ _returnvalue_2 -3e+01))
  (Transformation|SetRelativeLocation _sm_liftend1 (Math|Vector|MakeVector _returnvalue_4 (.y _relativelocation_2) (.z _relativelocation_2)) false false)
  (Transformation|SetRelativeLocation _sm_liftend2 (Math|Vector|MakeVector (* _returnvalue_4 -1.0) (.y _relativelocation) (.z _relativelocation)) false false)
  (Transformation|SetRelativeScale3D (Variables|Default|GetSM_LiftLaser1) (Math|Vector|MakeVector _returnvalue_3 1.0 1.0))
  (Transformation|SetRelativeScale3D (Variables|Default|GetSM_LiftLaser2) (Math|Vector|MakeVector _returnvalue_3 1.0 1.0)))

(event EventTick
  (params (DeltaSeconds :type Float%20%28single-precision%29))
  (bind _sm_lift (Variables|Default|GetSM_Lift))
  (bind _sm_lift_2 (Variables|Default|GetSM_Lift))
  (bind _relativelocation (Variables|/Script/Engine.SceneComponent|GetRelativeLocation _sm_lift))
  (bind _relativelocation_2 (Variables|/Script/Engine.SceneComponent|GetRelativeLocation _sm_lift_2))
  (if (Variables|Default|GetIsActive)
    (if (Variables|Default|GetReverse)
      (if (< (.x (Variables|/Script/Engine.SceneComponent|GetRelativeLocation (Variables|Default|GetSM_LiftEnd2))) (+ (.x (Variables|/Script/Engine.SceneComponent|GetRelativeLocation (Variables|Default|GetSM_Lift))) -1.9e+02))
        (Transformation|AddLocalOffset (Variables|Default|GetSM_Lift) (Math|Vector|MakeVector (* DeltaSeconds (Variables|Default|GetSpeed) -2e+02) 0.0 0.0) false false)
        (else
          (Utilities|FlowControl|DoOnce false :!label _label
            (:Completed
              (bind _moveend (Timeline|Lift PlayFromStart)
                (:Update
                  (Transformation|SetRelativeLocation _sm_lift (Math|Vector|MakeVector (+ (* _moveend -1.0) (.x _relativelocation)) (.y _relativelocation) (.z _relativelocation)) false false))
                (:Finished
                  (Utilities|FlowControl|Delay (Variables|Default|GetWaitTime))
                  (Variables|Default|SetReverse false)
                  (Utilities|FlowControl|Sequence
                    (:then_0
                      (goto _label Reset))
                    (:then_1
                      (Timeline|Lift SetNewTime)))))))))
      (elif (> (.x (Variables|/Script/Engine.SceneComponent|GetRelativeLocation (Variables|Default|GetSM_LiftEnd1))) (+ (.x (Variables|/Script/Engine.SceneComponent|GetRelativeLocation (Variables|Default|GetSM_Lift))) 1.9e+02))
        (Transformation|AddLocalOffset (Variables|Default|GetSM_Lift) (Math|Vector|MakeVector (* DeltaSeconds (Variables|Default|GetSpeed) 2e+02) 0.0 0.0) false false)
        (else
          (Utilities|FlowControl|DoOnce false :!label _label_2
            (:Completed
              (bind _moveend_2 (Timeline|Timeline_0 PlayFromStart)
                (:Update
                  (Transformation|SetRelativeLocation _sm_lift_2 (Math|Vector|MakeVector (+ _moveend_2 (.x _relativelocation_2)) (.y _relativelocation_2) (.z _relativelocation_2)) false false))
                (:Finished
                  (Utilities|FlowControl|Delay (Variables|Default|GetWaitTime))
                  (Variables|Default|SetReverse true)
                  (Utilities|FlowControl|Sequence
                    (:then_0
                      (goto _label_2 Reset))
                    (:then_1
                      (Timeline|Timeline_0 SetNewTime))))))))))))

(fn ConstructionScript)