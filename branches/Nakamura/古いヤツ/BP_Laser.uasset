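; BP_Laser is a laser barrier made of two poles with evenly stacked laser lines, sized by Width, Height and LaserQty.
; On BeginPlay it moves the poles apart to match Width, then stretches and raises them to match Height.
; It then spawns LaserQty BP_LaserLine actors spaced up the height and scaled to the width.
; The construction script is empty, so this layout is built only at runtime.
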(event EventBeginPlay
  (bind _returnvalue (Transformation|GetActorTransform))
  (bind _sm_leftpole (Variables|Default|GetSM_LeftPole))
  (bind _sm_rightpole (Variables|Default|GetSM_RightPole))
  (bind _height (Variables|Default|GetHeight))
  (bind _height_2 (Variables|Default|GetHeight))
  (bind _returnvalue_2 (Transformation|GetRelativeTransform _sm_rightpole))
  (bind _returnvalue_3 (Transformation|GetRelativeTransform _sm_leftpole))
  (Transformation|SetRelativeTransform _sm_leftpole (Math|Transform|MakeTransform (Math|Vector|MakeVector (/ (Variables|Default|GetWidth) 2.0) (.y (.location _returnvalue_3)) (+ (.z (.location _returnvalue_3)) (* 5e+01 (- _height_2 1.0)))) (.rotation _returnvalue_3) (Math|Vector|MakeVector (.x (.scale _returnvalue_3)) (.y (.scale _returnvalue_3)) _height_2)) false false)
  (Transformation|SetRelativeTransform _sm_rightpole (Math|Transform|MakeTransform (Math|Vector|MakeVector (/ (Variables|Default|GetWidth) -2.0) (.y (.location _returnvalue_2)) (+ (.z (.location _returnvalue_2)) (* 5e+01 (- _height 1.0)))) (.rotation _returnvalue_2) (Math|Vector|MakeVector (.x (.scale _returnvalue_2)) (.y (.scale _returnvalue_2)) _height)) false false)
  (for _index (range 1 (Math|Float|Truncate (Variables|Default|GetLaserQty)))
    (Game|SpawnActorfromClass "/Game/BP_LaserLine.BP_LaserLine_C" (Math|Transform|MakeTransform (Math|Vector|MakeVector (.x (.location _returnvalue)) (.y (.location _returnvalue)) (+ (* (Math|Conversions|ToFloat(Integer) _index) (/ (* (Variables|Default|GetHeight) 1e+02) (Variables|Default|GetLaserQty))) (.z (.location _returnvalue)) -2.0)) (.rotation _returnvalue) (Math|Vector|MakeVector (/ (Variables|Default|GetWidth) 4e+02) (.y (.scale _returnvalue)) (.z (.scale _returnvalue)))) "Undefined" 0 0)))

(fn ConstructionScript)