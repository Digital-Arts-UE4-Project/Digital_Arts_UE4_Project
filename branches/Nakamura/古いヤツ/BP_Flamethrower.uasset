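; Flamethrower actor that repeatedly spawns BP_Fire at its own transform, with a roll offset, in one of four modes chosen by Type.
; BeginPlay starts a looping timer for Full Time, Interval, Contact or Switch.
; Interval alternates bursts and pauses, while Contact re-enables fire on sphere overlap, both using a delayed ActionStop to set IsStop.
; Switch fires while IsStop is false, which FlameON_OFF toggles.
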(event EventBeginPlay
  (switch Utilities|FlowControl|Switch|SwitchonE_FlamethrowerType (Variables|Default|GetType)
    (:NewEnumerator0
      (Utilities|Time|SetTimerbyFunctionName 0 "FullTime" (Variables|Default|GetSpawnTime) true))
    (:NewEnumerator1
      (Utilities|Time|SetTimerbyFunctionName 0 "Interval" (+ (Variables|Default|GetActionTime) (Variables|Default|GetStopTime)) true))
    (:NewEnumerator2
      (Utilities|Time|SetTimerbyFunctionName 0 "Contact" (Variables|Default|GetSpawnTime) true))
    (:NewEnumerator3
      (Utilities|Time|SetTimerbyFunctionName 0 "Switch" (Variables|Default|GetSpawnTime) true))))

(event Custom|FullTime
  (bind _returnvalue (Transformation|GetActorTransform))
  (bind (_location _rotation _scale) (Math|Transform|BreakTransform _returnvalue))
  (Game|SpawnActorfromClass "/Game/BP_Fire.BP_Fire_C" (Math|Transform|MakeTransform _location (Math|Rotator|MakeRotator (+ (.roll _rotation) 1.7e+02) (.pitch _rotation) (.yaw _rotation)) _scale) "Undefined" self 0))

(event Custom|Interval
  (bind _returnvalue (Transformation|GetActorTransform))
  (bind (_location _rotation _scale) (Math|Transform|BreakTransform _returnvalue))
  (Variables|Default|SetIsStop false)
  (Utilities|Time|SetTimerbyFunctionName 0 "ActionStop" 0.001)
  (if (not (Variables|Default|GetIsStop)) :!label _label
    (Game|SpawnActorfromClass "/Game/BP_Fire.BP_Fire_C" (Math|Transform|MakeTransform _location (Math|Rotator|MakeRotator (+ (.roll _rotation) 1.7e+02) (.pitch _rotation) (.yaw _rotation)) _scale) "Undefined" 0 0)
    (Utilities|FlowControl|Delay (Variables|Default|GetSpawnTime))
    (goto _label)))

(event OnComponentBeginOverlap(Sphere)
  (params (OtherActor :type Actor%20Object%20Reference) (OtherComp :type Primitive%20Component%20Object%20Reference) (OtherBodyIndex :type Integer) (bFromSweep :type Boolean) (SweepResult :type Hit%20Result%20Structure%20%28by%20ref%29))
  (if (Variables|Default|GetIsTypeContact)
    (Variables|Default|SetIsStop false)))

(event Custom|Contact
  (bind _returnvalue (Transformation|GetActorTransform))
  (bind (_location _rotation _scale) (Math|Transform|BreakTransform _returnvalue))
  (Variables|Default|SetIsTypeContact true)
  (if (not (Variables|Default|GetIsStop))
    (Utilities|Time|SetTimerbyFunctionName 0 "ActionStop" 0.01)
    (if (not (Variables|Default|GetIsStop))
      (Game|SpawnActorfromClass "/Game/BP_Fire.BP_Fire_C" (Math|Transform|MakeTransform _location (Math|Rotator|MakeRotator (+ (.roll _rotation) 1.7e+02) (.pitch _rotation) (.yaw _rotation)) _scale) "Undefined" 0 0))))

(event Custom|FlameON_OFF
  (if (Variables|Default|GetIsTypeSwitch)
    (if (Variables|Default|GetIsStop)
      (Variables|Default|SetIsStop false)
      (else
        (Variables|Default|SetIsStop true)))))

(event Custom|Switch
  (bind _returnvalue (Transformation|GetActorTransform))
  (bind (_location _rotation _scale) (Math|Transform|BreakTransform _returnvalue))
  (Variables|Default|SetIsTypeSwitch true)
  (if (not (Variables|Default|GetIsStop))
    (Game|SpawnActorfromClass "/Game/BP_Fire.BP_Fire_C" (Math|Transform|MakeTransform _location (Math|Rotator|MakeRotator (+ (.roll _rotation) 1.7e+02) (.pitch _rotation) (.yaw _rotation)) _scale) "Undefined" 0 0)))

(event Custom|ActionStop
  (Utilities|FlowControl|Delay (Variables|Default|GetActionTime))
  (Variables|Default|SetIsStop true))

(fn ConstructionScript)