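; BP_Lift is a gimmick platform that shuttles back and forth along its local X axis between two end pieces, switched by GimmickON and GimmickOFF.
; The construction script positions the ends and scales both laser meshes from Length, and sets the initial moving state from IsActive.
; While moving, Tick offsets the lift at Speed, drops to a fixed rate near each end, then waits WaitTime before flipping Reverse.
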(event EventTick
  (params (DeltaSeconds :type Float%20%28single-precision%29))
  (bind _sm_lift (Variables|Default|GetSM_Lift))
  (bind _sm_liftend1 (Variables|Default|GetSM_LiftEnd1))
  (bind _sm_liftend2 (Variables|Default|GetSM_LiftEnd2))
  (bind _sm_lift_2 (Variables|Default|GetSM_Lift))
  (bind _relativelocation (Variables|/Script/Engine.SceneComponent|GetRelativeLocation _sm_liftend1))
  (bind _relativelocation_2 (Variables|/Script/Engine.SceneComponent|GetRelativeLocation _sm_lift))
  (bind _relativelocation_3 (Variables|/Script/Engine.SceneComponent|GetRelativeLocation _sm_liftend2))
  (bind _relativelocation_4 (Variables|/Script/Engine.SceneComponent|GetRelativeLocation _sm_lift_2))
  ;[1 1 1] 動作
  (if (Variables|Default|GetIsMove)
    (if (Variables|Default|GetReverse)
      (if (< (.x _relativelocation_3) (+ (.x _relativelocation_4) -2e+02))
        (Transformation|AddLocalOffset (Variables|Default|GetSM_Lift) (Math|Vector|MakeVector (* DeltaSeconds (Variables|Default|GetSpeed) -2e+02) 0.0 0.0) false false)
        (elif (<= (.x _relativelocation_3) (+ (.x _relativelocation_4) -9e+01))
          (Transformation|AddLocalOffset (Variables|Default|GetSM_Lift) (Math|Vector|MakeVector (* DeltaSeconds -1e+02) 0.0 0.0) false false)
          (else
            (Transformation|AddLocalOffset (Variables|Default|GetSM_Lift) (Math|Vector|MakeVector 0.0 0.0 0.0) false false)
            (Utilities|FlowControl|Delay (Variables|Default|GetWaitTime))
            (Variables|Default|SetReverse false))))
      (elif (> (.x _relativelocation) (+ (.x _relativelocation_2) 2e+02))
        (Transformation|AddLocalOffset (Variables|Default|GetSM_Lift) (Math|Vector|MakeVector (* DeltaSeconds (Variables|Default|GetSpeed) 2e+02) 0.0 0.0) false false)
        (elif (>= (.x _relativelocation) (+ (.x _relativelocation_2) 9e+01))
          (Transformation|AddLocalOffset (Variables|Default|GetSM_Lift) (Math|Vector|MakeVector (* DeltaSeconds 1e+02) 0.0 0.0) false false)
          (else
            (Transformation|AddLocalOffset (Variables|Default|GetSM_Lift) (Math|Vector|MakeVector 0.0 0.0 0.0) false false)
            (Utilities|FlowControl|Delay (Variables|Default|GetWaitTime))
            (Variables|Default|SetReverse true)))))))

(event EventGimmickON
  ;[1 1 1] ギミックのＯＮ／ＯＦＦ
  (Variables|Default|SetIsMove true))

(event EventGimmickOFF
  ;[1 1 1] ギミックのＯＮ／ＯＦＦ
  (Variables|Default|SetIsMove false))

(fn ConstructionScript
  (bind _length (Variables|Default|GetLength))
  (bind _sm_liftend1 (Variables|Default|GetSM_LiftEnd1))
  (bind _sm_liftend2 (Variables|Default|GetSM_LiftEnd2))
  (bind _length_2 (Variables|Default|GetLength))
  (bind _returnvalue (/ _length 2.0))
  (bind _returnvalue_2 (* _length_2 1e+02))
  (bind _relativelocation (Variables|/Script/Engine.SceneComponent|GetRelativeLocation _sm_liftend2))
  (bind _relativelocation_2 (Variables|/Script/Engine.SceneComponent|GetRelativeLocation _sm_liftend1))
  (bind _returnvalue_3 (- _returnvalue 0.1))
  (bind _returnvalue_4 (+ _returnvalue_2 -3e+01))
  ;[1 1 1] 初期設定
  (Transformation|SetRelativeLocation _sm_liftend1 (Math|Vector|MakeVector _returnvalue_4 (.y _relativelocation_2) (.z _relativelocation_2)) false false)
  (Transformation|SetRelativeLocation _sm_liftend2 (Math|Vector|MakeVector (* _returnvalue_4 -1.0) (.y _relativelocation) (.z _relativelocation)) false false)
  (Transformation|SetRelativeScale3D (Variables|Default|GetSM_LiftLaser1) (Math|Vector|MakeVector _returnvalue_3 1.0 1.0))
  (Transformation|SetRelativeScale3D (Variables|Default|GetSM_LiftLaser2) (Math|Vector|MakeVector _returnvalue_3 1.0 1.0))
  (if (Variables|Default|GetIsActive)
    (Variables|Default|SetIsMove true)
    (else
      (Variables|Default|SetIsMove false))))