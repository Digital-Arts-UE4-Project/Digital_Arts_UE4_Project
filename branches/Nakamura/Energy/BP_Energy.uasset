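; BP_Energy is an energy object that floats and rotates on a timeline until it switches to physics, then bursts into smaller pieces when hit.
; PhysicsChenge stops the float by setting IsPhysics and enables physics simulation on all static meshes under Main.
; Once in physics mode, the first Hit spawns Count BP_MinEnergy actors, scaled from Size and randomly jittered around the hit location, then destroys the actor.
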(event Custom|PhysicsChenge
  ;[1 1 1] 物理エンジンのOFF
  (for _array_element (Components|GetChildrenComponents (Variables|Default|Getmain) true)
    (bind _asstatic_mesh_component (Utilities|Casting|CastToStaticMeshComponent _array_element))
    (Utilities|Array|Add (Variables|Default|GetSM_Array) _asstatic_mesh_component))
  (Variables|Default|SetIsPhysics true)
  (for _array_element_2 (Variables|Default|GetSM_Array)
    (Physics|SetSimulatePhysics _array_element_2 true)))

(event EventBeginPlay
  (bind _main (Variables|Default|Getmain))
  (bind _returnvalue (Transformation|GetRelativeTransform _main))
  ;[1 1 1] 浮遊
  (bind (_direction _locationz _rotetion) (Timeline|Timeline_0 Play)
    (:Update
      (if (not (Variables|Default|GetIsPhysics))
        (Transformation|SetRelativeTransform _main (Math|Transform|MakeTransform (Math|Vector|MakeVector (.x (.location _returnvalue)) (.y (.location _returnvalue)) (+ (.z (.location _returnvalue)) _locationz)) (Math|Rotator|MakeRotator 0.0 _rotetion _rotetion) (.scale _returnvalue)) false false)))))

(event Collision|EventHit
  (params (MyComp :type Primitive%20Component%20Object%20Reference) (Other :type Actor%20Object%20Reference) (OtherComp :type Primitive%20Component%20Object%20Reference) (bSelfMoved :type Boolean) (HitLocation :type Vector) (HitNormal :type Vector) (NormalImpulse :type Vector) (Hit :type Hit%20Result%20Structure%20%28by%20ref%29))
  (bind _returnvalue (Math|Random|RandomFloatinRange -5.0 5.0))
  (bind _size (Variables|Default|GetSize))
  (bind _returnvalue_2 (/ _size 1e+01))
  ;[1 1 1] 消去
  (if (Variables|Default|GetIsPhysics)
    (Utilities|FlowControl|DoOnce false
      (:Completed
        (for _index (range 1 (Variables|Default|Getcount))
          (Game|SpawnActorfromClass "/Game/Blueprint/Gimmicks/Blueprint/BP_MinEnergy.BP_MinEnergy_C" (Math|Transform|MakeTransform (+ HitLocation (Math|Vector|MakeVector _returnvalue _returnvalue _returnvalue)) "0, 0, 0" (Math|Vector|MakeVector _returnvalue_2 _returnvalue_2 _returnvalue_2)) "Undefined" 0 0))
        (Actor|DestroyActor)))))

(fn ConstructionScript)